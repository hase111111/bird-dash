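; BP_JumpPad_dark is a jump pad variant that launches itself, spinning in pitch, when an actor tagged Player first overlaps its mesh.
; A DoOnce on overlap enables Tick, raises a physics flag, seeds vertical velocity and replaces its Tags with TagEmpty.
; Tick hand-rolls the motion per frame without delta-time scaling, adding acceleration to velocity and offsetting Z without sweep.
; It applies no impulse to the player.
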(event OnComponentBeginOverlap(StaticMesh)
  (params (OverlappedComponent :type Primitive%20Component%20Object%20Reference) (OtherActor :type Actor%20Object%20Reference) (OtherComp :type Primitive%20Component%20Object%20Reference) (OtherBodyIndex :type Integer) (bFromSweep :type Boolean) (SweepResult :type Hit%20Result%20Structure%20%28by%20ref%29))
  (Utilities|IsValid OtherActor
    (:Is%20Valid
      (if (Actor|ActorHasTag OtherActor (Variables|Default|GetPlayer)) ; ヒットしたら
        (Utilities|FlowControl|DoOnce false
          (:Completed
            (Actor|Tick|SetActorTickEnabled true)
            (Variables|Default|Setフラグ-物理演算開始 true)
            (Variables|Default|SetZvec 8.0)
            (Variables|Default|SetTags (Variables|Default|GetTag_empty))))))))

(event EventBeginPlay
  (Actor|Tick|SetActorTickEnabled false))

(event EventTick
  (params (DeltaSeconds :type Float%20%28single-precision%29))
  (bind _returnvalue (Transformation|GetActorRotation))
  (bind _returnvalue_2 (Transformation|GetActorLocation))
  (if (Variables|Default|Getフラグ-物理演算開始)
    (Variables|Default|SetZvec (+ (Variables|Default|GetZvec) (Variables|Default|GetZacc)))
    (Transformation|SetActorLocation (Math|Vector|MakeVector (.x _returnvalue_2) (.y _returnvalue_2) (+ (.z _returnvalue_2) (Variables|Default|GetZvec))) false false)
    (bind _output_get (Variables|Default|SetAnimation (Math|Rotator|MakeRotator (.roll _returnvalue) (+ (.pitch _returnvalue) (Variables|Default|Get回転速度)) (.yaw _returnvalue))))
    (Transformation|SetActorRotation _output_get)))

(fn ConstructionScript)