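; BP_Obstacle_Bullet is a bullet obstacle that grows into view, then flies off once triggered.
; BeginPlay tags it as Obstacle and zeroes its scale, and Tick scales it up linearly over a configurable duration.
; Calling 移動開始 (start moving) sets a flag that makes Tick move it at constant speed along world negative Y.
; The first moving frame plays a gunshot sound and sets a short lifespan.
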(event EventBeginPlay
  (Variables|Default|SetTags (Variables|Default|GetObstacle))
  (Transformation|SetActorTransform (Math|Transform|MakeTransform (Transformation|GetActorLocation) "0, 0, 0" "0.000000,0.000000,0.000000")))

(event EventTick
  (params (DeltaSeconds :type Float%20%28single-precision%29))
  (Variables|Default|Set時間カウント (+ DeltaSeconds (Variables|Default|Get時間カウント)))
  (if (<= (/ (Variables|Default|Get時間カウント) (Variables|Default|Get元のサイズになるまで何秒)) 1.0)
    (Transformation|SetActorTransform (Math|Transform|MakeTransform (Transformation|GetActorLocation) "0, 0, 0" (* (Math|Vector|MakeVector 0.8 0.8 0.8) (/ (Variables|Default|Get時間カウント) (Variables|Default|Get元のサイズになるまで何秒))))))
  (if (Variables|Default|Get移動するか?)
    (Transformation|SetActorLocation (+ (Transformation|GetActorLocation) (Math|Vector|MakeVector 0.0 (* DeltaSeconds -1e+03) 0.0)) false false)
    (Utilities|FlowControl|DoOnce false
      (:Completed
        (Actor|SetLifeSpan 3.0)
        (Audio|PlaySoundatLocation "/Game/Sound/SE/銃をうつ.銃をうつ" (Transformation|GetActorLocation) "0, 0, 0" 1.0 1.0 0.0 0 0 0 0)))))

(fn ConstructionScript)

(fn 移動開始
  (Variables|Default|Set移動するか? true))