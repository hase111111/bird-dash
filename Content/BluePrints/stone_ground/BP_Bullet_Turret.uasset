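; BP_Bullet_Turret is an obstacle turret that fires a single bullet as the player approaches along the Y axis.
; On BeginPlay it sets the Obstacle tag, then Tick compares the player's Y position against two distance thresholds.
; The outer threshold pre-spawns a BP_Obstacle_Bullet just below the turret via SpawnAIFromClass.
; The inner threshold calls 移動開始 to start its movement, with each step guarded by DoOnce.
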(event EventBeginPlay
  (Variables|Default|SetTags (Variables|Default|GetObstacle)))

(event EventTick
  (params (DeltaSeconds :type Float%20%28single-precision%29))
  (if (not (Variables|Default|Get弾生成済み))
    (if (> (.y (Transformation|GetActorLocation (Game|Player|GetPlayerPawn 0))) (Utilities|Operators|Subtract (.y (Transformation|GetActorLocation)) (Variables|Default|Get弾丸生成距離) (Variables|Default|Getどのくらい近づいたら撃つか)))
      (Utilities|FlowControl|DoOnce false
        (:Completed
          (bind _returnvalue (AI|SpawnAIFromClass "/Game/BluePrints/stone_ground/BP_Obstacle_Bullet.BP_Obstacle_Bullet_C" 0 (+ (Transformation|GetActorLocation) (Math|Vector|MakeVector 0.0 0.0 -5e+01)) "0, 0, 0" true 0))
          (Variables|Default|Set弾 _returnvalue)
          (Variables|Default|Set弾生成済み true))))
    (elif (> (.y (Transformation|GetActorLocation (Game|Player|GetPlayerPawn 0))) (- (.y (Transformation|GetActorLocation)) (Variables|Default|Getどのくらい近づいたら撃つか)))
      (Utilities|FlowControl|DoOnce false
        (:Completed
          (bind _asbp_obstacle_bullet (Utilities|Casting|CastToBP_Obstacle_Bullet (Variables|Default|Get弾)))
          (Default|移動開始 _asbp_obstacle_bullet))))))

(fn ConstructionScript)