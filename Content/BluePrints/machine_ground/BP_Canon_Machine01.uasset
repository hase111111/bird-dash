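; Ground cannon machine that fires a one-time volley of BP_Neji_Canon pawns once the player's Y position passes 1000 units short of it.
; Tick triggers a DoOnce chain over eight landing points, spawning each pawn 75 units behind the actor's yaw, passing it the target's X/Y and waiting DelayTime.
; Points with non-positive Y are skipped, except 着弾地点02, whose unwired False branch ends the volley.
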(event Collision|EventActorBeginOverlap
  (params (OtherActor :type Actor%20Object%20Reference)))

(event EventTick
  (params (DeltaSeconds :type Float%20%28single-precision%29))
  (bind _着弾地点00 (Variables|Default|Get着弾地点00))
  (bind _着弾地点01 (Variables|Default|Get着弾地点01))
  (bind _着弾地点02 (Variables|Default|Get着弾地点02))
  (bind _着弾地点03 (Variables|Default|Get着弾地点03))
  (bind _着弾地点04 (Variables|Default|Get着弾地点04))
  (bind _着弾地点05 (Variables|Default|Get着弾地点05))
  (bind _着弾地点06 (Variables|Default|Get着弾地点06))
  (bind _着弾地点07 (Variables|Default|Get着弾地点07))
  (if (< (.y (Transformation|GetActorLocation)) (+ (.y (Transformation|GetActorLocation (Game|GetPlayerCharacter 0))) 1e+03))
    (Utilities|FlowControl|DoOnce false
      (:Completed
        (if (> (.y _着弾地点00) 0.0)
          (bind _newparam (CallFunction|発射場所))
          (bind _returnvalue (AI|SpawnAIFromClass "/Game/BluePrints/machine_ground/BP_Neji_Canon.BP_Neji_Canon_C" 0 _newparam "0, 0, 0" false 0))
          (bind _asbp_neji_canon (Utilities|Casting|CastToBP_Neji_Canon _returnvalue))
          (Default|着弾地点セット _asbp_neji_canon (.x _着弾地点00) (.y _着弾地点00))
          (Utilities|FlowControl|Delay (Variables|Default|Getdelay_time)))
        (if (> (.y _着弾地点01) 0.0)
          (bind _newparam_2 (CallFunction|発射場所))
          (bind _returnvalue_2 (AI|SpawnAIFromClass "/Game/BluePrints/machine_ground/BP_Neji_Canon.BP_Neji_Canon_C" 0 _newparam_2 "0, 0, 0" false 0))
          (bind _asbp_neji_canon_2 (Utilities|Casting|CastToBP_Neji_Canon _returnvalue_2))
          (Default|着弾地点セット _asbp_neji_canon_2 (.x _着弾地点01) (.y _着弾地点01))
          (Utilities|FlowControl|Delay (Variables|Default|Getdelay_time)))
        (if (> (.y _着弾地点02) 0.0)
          (bind _newparam_3 (CallFunction|発射場所))
          (bind _returnvalue_3 (AI|SpawnAIFromClass "/Game/BluePrints/machine_ground/BP_Neji_Canon.BP_Neji_Canon_C" 0 _newparam_3 "0, 0, 0" false 0))
          (bind _asbp_neji_canon_3 (Utilities|Casting|CastToBP_Neji_Canon _returnvalue_3))
          (Default|着弾地点セット _asbp_neji_canon_3 (.x _着弾地点02) (.y _着弾地点02))
          (Utilities|FlowControl|Delay (Variables|Default|Getdelay_time))
          (if (> (.y _着弾地点03) 0.0)
            (bind _newparam_4 (CallFunction|発射場所))
            (bind _returnvalue_4 (AI|SpawnAIFromClass "/Game/BluePrints/machine_ground/BP_Neji_Canon.BP_Neji_Canon_C" 0 _newparam_4 "0, 0, 0" false 0))
            (bind _asbp_neji_canon_4 (Utilities|Casting|CastToBP_Neji_Canon _returnvalue_4))
            (Default|着弾地点セット _asbp_neji_canon_4 (.x _着弾地点03) (.y _着弾地点03))
            (Utilities|FlowControl|Delay (Variables|Default|Getdelay_time)))
          (if (> (.y _着弾地点04) 0.0)
            (bind _newparam_5 (CallFunction|発射場所))
            (bind _returnvalue_5 (AI|SpawnAIFromClass "/Game/BluePrints/machine_ground/BP_Neji_Canon.BP_Neji_Canon_C" 0 _newparam_5 "0, 0, 0" false 0))
            (bind _asbp_neji_canon_5 (Utilities|Casting|CastToBP_Neji_Canon _returnvalue_5))
            (Default|着弾地点セット _asbp_neji_canon_5 (.x _着弾地点04) (.y _着弾地点04))
            (Utilities|FlowControl|Delay (Variables|Default|Getdelay_time)))
          (if (> (.y _着弾地点05) 0.0)
            (bind _newparam_6 (CallFunction|発射場所))
            (bind _returnvalue_6 (AI|SpawnAIFromClass "/Game/BluePrints/machine_ground/BP_Neji_Canon.BP_Neji_Canon_C" 0 _newparam_6 "0, 0, 0" false 0))
            (bind _asbp_neji_canon_6 (Utilities|Casting|CastToBP_Neji_Canon _returnvalue_6))
            (Default|着弾地点セット _asbp_neji_canon_6 (.x _着弾地点05) (.y _着弾地点05))
            (Utilities|FlowControl|Delay (Variables|Default|Getdelay_time)))
          (if (> (.y _着弾地点06) 0.0)
            (bind _newparam_7 (CallFunction|発射場所))
            (bind _returnvalue_7 (AI|SpawnAIFromClass "/Game/BluePrints/machine_ground/BP_Neji_Canon.BP_Neji_Canon_C" 0 _newparam_7 "0, 0, 0" false 0))
            (bind _asbp_neji_canon_7 (Utilities|Casting|CastToBP_Neji_Canon _returnvalue_7))
            (Default|着弾地点セット _asbp_neji_canon_7 (.x _着弾地点06) (.y _着弾地点06))
            (Utilities|FlowControl|Delay (Variables|Default|Getdelay_time)))
          (if (> (.y _着弾地点07) 0.0)
            (bind _newparam_8 (CallFunction|発射場所))
            (bind _returnvalue_8 (AI|SpawnAIFromClass "/Game/BluePrints/machine_ground/BP_Neji_Canon.BP_Neji_Canon_C" 0 _newparam_8 "0, 0, 0" false 0))
            (bind _asbp_neji_canon_8 (Utilities|Casting|CastToBP_Neji_Canon _returnvalue_8))
            (Default|着弾地点セット _asbp_neji_canon_8 (.x _着弾地点07) (.y _着弾地点07))
            (Utilities|FlowControl|Delay (Variables|Default|Getdelay_time))))))))

(fn ConstructionScript)

(fn 発射場所
  (bind _returnvalue (Transformation|GetActorLocation))
  (bind _returnvalue_2 (Transformation|GetActorRotation))
  (return (+ (Math|Vector|MakeVector (* (Math|Trig|Cos(Degrees) (.yaw _returnvalue_2)) -75.0) (* (Math|Trig|Sin(Degrees) (.yaw _returnvalue_2)) -75.0) 0.0) (Math|Vector|MakeVector (.x _returnvalue) (.y _returnvalue) (+ (.z _returnvalue) 0.0)))))