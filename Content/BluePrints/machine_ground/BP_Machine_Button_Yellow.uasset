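; Yellow machine button actor that the player presses by overlapping its capsule, which tells the level's BP_Button_Controller to turn yellow on.
; It finds the controller on BeginPlay and polls its yellow state every Tick, reacting only when that state changes.
; The on and off looks are shown by toggling visibility between two static meshes, so the button mirrors the controller's shared state.
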(event OnComponentBeginOverlap(Capsule)
  (params (OverlappedComponent :type Primitive%20Component%20Object%20Reference) (OtherActor :type Actor%20Object%20Reference) (OtherComp :type Primitive%20Component%20Object%20Reference) (OtherBodyIndex :type Integer) (bFromSweep :type Boolean) (SweepResult :type Hit%20Result%20Structure%20%28by%20ref%29))
  (bind _button_controller_ref (Variables|Default|Getbutton_controller_ref))
  (Utilities|IsValid OtherActor
    (:Is%20Valid
      (if (Actor|ActorHasTag OtherActor "player")
        (Utilities|IsValid _button_controller_ref
          (:Is%20Valid
            (Default|SetYellowon _button_controller_ref)))))))

(event EventBeginPlay
  (bind _returnvalue (Actor|GetActorOfClass "/Game/BluePrints/machine_ground/BP_Button_Controller.BP_Button_Controller_C"))
  (bind _output_get (Variables|Default|Setbutton_controller_ref _returnvalue))
  (bind _newparam (Default|GetYellowON _output_get))
  (bind _output_get_2 (Variables|Default|Setyellow_is_on _newparam))
  (if _output_get_2
    (CallFunction|ChangeYellowON)
    (else
      (CallFunction|ChangeYellowOFF))))

(event EventTick
  (params (DeltaSeconds :type Float%20%28single-precision%29))
  (bind _button_controller_ref (Variables|Default|Getbutton_controller_ref))
  (Utilities|IsValid _button_controller_ref
    (:Is%20Valid
      (bind _newparam (Default|GetYellowON _button_controller_ref))
      (if (Class|KismetMathLibrary|XORBoolean _newparam (Variables|Default|Getyellow_is_on))
        (bind _output_get (Variables|Default|Setyellow_is_on _newparam))
        (if _output_get
          (CallFunction|ChangeYellowON)
          (else
            (CallFunction|ChangeYellowOFF)))))))

(fn ConstructionScript)

(fn ChangeYellowON
  (Rendering|SetVisibility (Variables|Default|GetStaticMesh1) true false)
  (Rendering|SetVisibility (Variables|Default|GetStaticMesh) false false))

(fn ChangeYellowOFF
  (Rendering|SetVisibility (Variables|Default|GetStaticMesh1) false false)
  (Rendering|SetVisibility (Variables|Default|GetStaticMesh) true false))