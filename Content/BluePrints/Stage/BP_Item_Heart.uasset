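; Collectible heart pickup for a stage, one of three slots identified by an Index that SetIndex clamps to a valid range.
; Until collected, Tick bobs it on a sine wave above its starting height and spins it slowly.
; Overlap by a "player"-tagged actor stops the bob and speeds up the spin.
; A DoOnce then plays a sound, sets a short lifespan and sets the matching heart-acquired flag in BP_My_Player_State.
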(event OnComponentBeginOverlap(StaticMesh)
  (params (OverlappedComponent :type Primitive%20Component%20Object%20Reference) (OtherActor :type Actor%20Object%20Reference) (OtherComp :type Primitive%20Component%20Object%20Reference) (OtherBodyIndex :type Integer) (bFromSweep :type Boolean) (SweepResult :type Hit%20Result%20Structure%20%28by%20ref%29))
  ;[1 1 1] アイテム取得処理
  (Utilities|IsValid OtherActor
    (:Is%20Valid
      (if (Actor|ActorHasTag OtherActor "player")
        (Variables|Default|Setalready_get true)))))

(event EventBeginPlay
  (Variables|Default|Setfirst_z_pos (.z (Transformation|GetActorLocation))))

(event EventTick
  (params (DeltaSeconds :type Float%20%28single-precision%29))
  (bind _returnvalue (Game|GetPlayerState 0))
  (Variables|Default|Setcount (+ DeltaSeconds (Variables|Default|Getcount)))
  (if (Variables|Default|Getalready_get)
    ;[1 1 1] 取得後
    (CallFunction|PlayRotaionAnime DeltaSeconds (* (Variables|Default|Getrot_speed) 15.0))
    (Utilities|FlowControl|DoOnce false
      (:Completed
        (Actor|SetLifeSpan 3.0)
        (Audio|PlaySound2D "/Game/Sound/SE/魔王魂_効果音_システム46_Cue.魔王魂_効果音_システム46_Cue" 1.0 1.0 0.0 0 0)
        ;[1 1 1] Player stateに知らせる
        (switch int (Variables|Default|Getindex)
          (:0
            (bind _asbp_my_player_state (Utilities|Casting|CastToBP_My_Player_State _returnvalue))
            (Variables|/Game/BluePrints/Stage/BP_My_Player_State.BP_My_Player_State_C|Setハート取得済み1 _asbp_my_player_state true))
          (:1
            (bind _asbp_my_player_state_2 (Utilities|Casting|CastToBP_My_Player_State _returnvalue))
            (Variables|/Game/BluePrints/Stage/BP_My_Player_State.BP_My_Player_State_C|Setハート取得済み2 _asbp_my_player_state_2 true))
          (:2
            (bind _asbp_my_player_state_3 (Utilities|Casting|CastToBP_My_Player_State _returnvalue))
            (Variables|/Game/BluePrints/Stage/BP_My_Player_State.BP_My_Player_State_C|Setハート取得済み3 _asbp_my_player_state_3 true)))))
    (else
      ;[1 1 1] 取得前
      (CallFunction|PlayFlyAnime DeltaSeconds)
      (CallFunction|PlayRotaionAnime DeltaSeconds (Variables|Default|Getrot_speed)))))

(fn ConstructionScript)

(fn SetIndex
  (params (number0・1・２ :type Integer))
  (bind _output_get (Variables|Default|Setindex number0・1・２))
  (if (>= _output_get 3)
    (Variables|Default|Setindex 2)
    (elif (<= (Variables|Default|Getindex) -1)
      (Variables|Default|Setindex 0))))

(fn PlayFlyAnime
  (params (delta :type Float%20%28double-precision%29))
  (bind _returnvalue (Transformation|GetActorLocation))
  (Transformation|SetActorLocation (Math|Vector|MakeVector (.x _returnvalue) (.y _returnvalue) (+ (Variables|Default|Getfirst_z_pos) (Variables|Default|Getamplitude) (* (Math|Trig|Sin(Degrees) (* (Variables|Default|Getcount) 9e+01)) (Variables|Default|Getamplitude)))) false false))

(fn PlayRotaionAnime
  (params (delta :type Float%20%28double-precision%29) (速度 :type Float%20%28double-precision%29))
  (Transformation|SetActorRotation (Math|Rotator|MakeRotator 0.0 0.0 (+ (.yaw (Transformation|GetActorRotation)) (* 速度 delta)))))