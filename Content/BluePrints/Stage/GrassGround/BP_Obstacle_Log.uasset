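; Rolling log obstacle for the GrassGround stage that sets off toward the approaching player along the negative Y axis.
; It tags itself on BeginPlay, then Tick waits until player 0's Y position passes the log's Y minus MoveDistance.
; Once triggered, it sets a 10-second lifespan and rolls and slides by fixed per-frame steps, without delta-time scaling or collision sweep.
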(event EventBeginPlay
  (Variables|Default|SetTags (Variables|Default|Getobstacle_tag)))

(event EventTick
  (params (DeltaSeconds :type Float%20%28single-precision%29))
  (bind _returnvalue (Transformation|GetActorLocation))
  (if (Variables|Default|Getis_moved)
    (Transformation|SetActorRotation (Math|Rotator|MakeRotator (+ (.roll (Transformation|GetActorRotation)) -3.0) 0.0 0.0))
    (Transformation|SetActorLocation (Math|Vector|MakeVector (.x _returnvalue) (+ (.y _returnvalue) -5.0) (.z _returnvalue)) false false)
    (elif (> (.y (Transformation|GetActorLocation (Game|GetPlayerCharacter 0))) (- (.y (Transformation|GetActorLocation)) (Variables|Default|Getmove_distance)))
      (Variables|Default|Setis_moved true)
      (Actor|SetLifeSpan 1e+01))))

(fn ConstructionScript)