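; BP_Obstacle_Robot_01 is a moving robot obstacle in the MachineGround stage that activates based on the player's position.
; BeginPlay assigns its actor tags from a variable.
; Each Tick, while player 0's Y exceeds the robot's Y minus 600, it teleport-free moves by a vector scaled by a speed variable, without sweep or frame-time scaling.
; A DoOnce plays a 2D machine sound on the first move.
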(event EventBeginPlay
  (Variables|Default|SetTags (Variables|Default|GetTags_0)))

(event EventTick
  (params (DeltaSeconds :type Float%20%28single-precision%29))
  (if (< (- (.y (Transformation|GetActorLocation)) 6e+02) (.y (Transformation|GetActorLocation (Game|GetPlayerCharacter 0))))
    (Transformation|SetActorLocation (+ (* (Variables|Default|GetNewVar_0) (Variables|Default|Get移動速度)) (Transformation|GetActorLocation)) false false)
    (Utilities|FlowControl|DoOnce false
      (:Completed
        (Audio|PlaySound2D "/Game/Sound/SE/機械音.機械音" 1.0 1.0 0.0 0 0)))))

(fn ConstructionScript)