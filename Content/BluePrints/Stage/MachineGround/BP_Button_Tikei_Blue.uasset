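; BP_Button_Tikei_Blue is a MachineGround stage terrain actor that moves vertically with the button controller's yellow state, despite its Blue name.
; On BeginPlay it stores its start location and finds BP_Button_Controller, then polls YellowON every Tick.
; While YellowON, VInterpTo eases it slowly toward a fixed world Z at its original X/Y.
; Otherwise it returns much faster to its start location.
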(event EventBeginPlay
  (Variables|Default|Set最初の座標 (Transformation|GetActorLocation))
  (bind _returnvalue (Actor|GetActorOfClass "/Game/BluePrints/Stage/MachineGround/BP_Button_Controller.BP_Button_Controller_C"))
  (bind _output_get (Variables|Default|Setコントローラの参照 _returnvalue))
  (bind _newparam (Default|GetYellowON _output_get))
  (Variables|Default|SetYellow%20ON _newparam))

(event EventTick
  (params (DeltaSeconds :type Float%20%28single-precision%29))
  (bind _最初の座標 (Variables|Default|Get最初の座標))
  (bind _コントローラの参照 (Variables|Default|Getコントローラの参照))
  (if (Variables|Default|GetYellow%20ON)
    (Transformation|SetActorLocation (Math|Interpolation|VInterpTo (Transformation|GetActorLocation) (Math|Vector|MakeVector (.x _最初の座標) (.y _最初の座標) 2e+03) (Utilities|Time|GetWorldDeltaSeconds) 1.0) false false)
    (else
      (Transformation|SetActorLocation (Math|Interpolation|VInterpTo (Transformation|GetActorLocation) (Variables|Default|Get最初の座標) (Utilities|Time|GetWorldDeltaSeconds) 3e+01) false false)))
  (Utilities|IsValid _コントローラの参照
    (:Is%20Valid
      (bind _newparam (Default|GetYellowON _コントローラの参照))
      (if (Class|KismetMathLibrary|XORBoolean _newparam (Variables|Default|GetYellow%20ON))
        (Variables|Default|SetYellow%20ON _newparam)))))

(fn ConstructionScript)