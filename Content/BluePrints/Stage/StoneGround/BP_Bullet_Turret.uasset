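; Stage obstacle turret that fires a single BP_Obstacle_Bullet as the player approaches along the Y axis.
; BeginPlay assigns its obstacle tag, and Tick compares the player pawn's Y position against two distance thresholds.
; At the farther threshold it spawns the bullet as an AI pawn slightly below itself and stores it.
; At ShotDistance it calls the bullet's 移動開始 (start movement), with each stage guarded by a DoOnce.
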(event EventBeginPlay
  (Variables|Default|SetTags (Variables|Default|Getobstacle_tag)))

(event EventTick
  (params (DeltaSeconds :type Float%20%28single-precision%29))
  (if (not (Variables|Default|Getalready_generated))
    (if (> (.y (Transformation|GetActorLocation (Game|Player|GetPlayerPawn 0))) (Utilities|Operators|Subtract (.y (Transformation|GetActorLocation)) (Variables|Default|Getbullet_distance) (Variables|Default|Getshot_distance)))
      (Utilities|FlowControl|DoOnce false
        (:Completed
          (bind _returnvalue (AI|SpawnAIFromClass "/Game/BluePrints/Stage/StoneGround/BP_Obstacle_Bullet.BP_Obstacle_Bullet_C" 0 (+ (Transformation|GetActorLocation) (Math|Vector|MakeVector 0.0 0.0 -5e+01)) "0, 0, 0" true 0))
          (Variables|Default|Setbullet _returnvalue)
          (Variables|Default|Setalready_generated true))))
    (elif (> (.y (Transformation|GetActorLocation (Game|Player|GetPlayerPawn 0))) (- (.y (Transformation|GetActorLocation)) (Variables|Default|Getshot_distance)))
      (Utilities|FlowControl|DoOnce false
        (:Completed
          (bind _asbp_obstacle_bullet (Utilities|Casting|CastToBP_Obstacle_Bullet (Variables|Default|Getbullet)))
          (Default|移動開始 _asbp_obstacle_bullet))))))

(fn ConstructionScript)