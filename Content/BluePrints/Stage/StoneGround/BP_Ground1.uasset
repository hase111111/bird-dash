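; BP_Ground1 is a stage ground actor that slides back and forth along the world X axis.
; BeginPlay stores the starting X and assigns the actor's tags.
; Tick accumulates time and sets X to that origin plus a degree-based sine wave, shaped by speed, phase offset and amplitude variables.
; Y and Z are kept, and the move neither sweeps nor teleports.
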(event EventBeginPlay
  ;[1 1 1] 初期座標をセット
  (Variables|Default|Set初期x座標 (.x (Transformation|GetActorLocation)))
  (Variables|Default|SetTags (Variables|Default|GetTags_0)))

(event EventTick
  (params (DeltaSeconds :type Float%20%28single-precision%29))
  (bind _returnvalue (Transformation|GetActorLocation))
  ;[1 1 1] カウンターを進める
  (Variables|Default|Setcounter (+ DeltaSeconds (Variables|Default|Getcounter)))
  ;[1 1 1] 座標を設定
  (Transformation|SetActorLocation (Math|Vector|MakeVector (+ (* (Math|Trig|Sin(Degrees) (+ (* (Variables|Default|Getcounter) (Variables|Default|Get往復速度)) (Variables|Default|Get初期位相))) (Variables|Default|Get移動の横幅)) (Variables|Default|Get初期x座標)) (.y _returnvalue) (.z _returnvalue)) false false))

(fn ConstructionScript)