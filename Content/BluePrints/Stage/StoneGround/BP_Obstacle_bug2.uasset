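; BP_Obstacle_bug2 is a StoneGround stage obstacle, tagged Obstacle, that wanders randomly around its starting position.
; A randomly offset timer periodically picks a new target within configurable X/Y ranges at the starting height.
; Each tick it moves toward that target at constant speed without sweeping, smoothly turning to face its direction of travel by comparing against its previous position.
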(event EventBeginPlay
  (Variables|Default|SetTags (Variables|Default|GetObstacle))
  (bind _output_get (Variables|Default|Set初期座標 (Transformation|GetActorLocation)))
  (Variables|Default|Set移動先 _output_get)
  (Variables|Default|Setcounter (* (Math|Random|RandomFloat) (Variables|Default|Get移動位置を決める周期))))

(event EventTick
  (params (DeltaSeconds :type Float%20%28single-precision%29))
  (bind _returnvalue (Math|Random|RandomFloat))
  (bind _初期座標 (Variables|Default|Get初期座標))
  (bind _returnvalue_2 (- _returnvalue 0.5))
  (bind _returnvalue_3 (* _returnvalue_2 2.0))
  (bind _output_get (Variables|Default|Setcounter (+ DeltaSeconds (Variables|Default|Getcounter))))
  (if (> _output_get (Variables|Default|Get移動位置を決める周期))
    (Variables|Default|Setcounter 0.0)
    (Variables|Default|Set移動先 (Math|Vector|MakeVector (+ (* _returnvalue_3 (Variables|Default|Get移動範囲X)) (.x _初期座標)) (+ (* _returnvalue_3 (Variables|Default|Get移動範囲Y)) (.y _初期座標)) (.z _初期座標))))
  (Transformation|SetActorLocation (Math|Interpolation|VInterptoConstant (Transformation|GetActorLocation) (Variables|Default|Get移動先) (Utilities|Time|GetWorldDeltaSeconds) 2.5e+02) false false)
  (if (Utilities|Operators|NotEqual(!=) (Variables|Default|Get一瞬前の座標) (Transformation|GetActorLocation) 0.01)
    (Transformation|SetActorRotation (Math|Interpolation|RInterpTo (Transformation|GetActorRotation) (Math|Rotator|FindLookatRotation (Variables|Default|Get一瞬前の座標) (Transformation|GetActorLocation)) (Utilities|Time|GetWorldDeltaSeconds) 1e+01))
    (Variables|Default|Set一瞬前の座標 (Transformation|GetActorLocation))))

(fn ConstructionScript)