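; BP_Obstacle_Monster is a monster obstacle for the StoneGround stage that moves vertically as the player approaches along Y.
; BeginPlay tags it Obstacle and stores its starting position.
; Each Tick compares player Y to two thresholds before the monster, interpolating it below its start at the farther one, then above it at the nearer one.
; The first rise also sets AttackFlag through a DoOnce.
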(event EventBeginPlay
  (Variables|Default|SetTags (Variables|Default|GetObstacle))
  (Variables|Default|Set初期座標 (Transformation|GetActorLocation)))

(event EventTick
  (params (DeltaSeconds :type Float%20%28single-precision%29))
  (bind _returnvalue (Game|GetPlayerCharacter 0))
  (bind _returnvalue_2 (Transformation|GetActorLocation))
  (bind _初期座標 (Variables|Default|Get初期座標))
  (bind _初期座標_2 (Variables|Default|Get初期座標))
  (bind _returnvalue_3 (Transformation|GetActorLocation _returnvalue))
  (if (> (.y _returnvalue_3) (- (.y _returnvalue_2) 7.5e+02))
    (if (> (.y _returnvalue_3) (- (.y _returnvalue_2) 3.5e+02))
      (Transformation|SetActorLocation (Math|Interpolation|VInterpTo (Transformation|GetActorLocation) (Math|Vector|MakeVector (.x _初期座標) (.y _初期座標) (+ (.z _初期座標) 2e+02)) (Utilities|Time|GetWorldDeltaSeconds) 2.0) false false)
      (Utilities|FlowControl|DoOnce false
        (:Completed
          (Variables|Default|Setattack_flag true)))
      (else
        (Transformation|SetActorLocation (Math|Interpolation|VInterpTo (Transformation|GetActorLocation) (Math|Vector|MakeVector (.x _初期座標_2) (.y _初期座標_2) (- (.z _初期座標_2) 1e+02)) (Utilities|Time|GetWorldDeltaSeconds) 2.0) false false)))))

(fn ConstructionScript)