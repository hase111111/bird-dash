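; Player controller for stages that runs the start, pause, miss and goal screens around the player's BP_Wing_Bird.
; BeginPlay picks BGM from DT_Stage_List by level name and pre-creates the widgets.
; Tick polls the bird for miss or goal, firing each screen once through DoOnce.
; Flags gate confirm and menu input during animations; confirm starts the bird, drives the pause menu, restarts after misses, or saves the clear and hearts before returning to stage select.
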(event EventTick
  (params (DeltaSeconds :type Float%20%28single-precision%29))
  (bind _goal_value (Variables|Default|GetGoal_value))
  (bind _miss_value (Variables|Default|Getmiss_value))
  ;[1 1 1] ミスしたか?
  (bind _asbp_wing_bird (Utilities|Casting|CastToBP_Wing_Bird (Pawn|GetControlledPawn)))
  (if (Variables|/Game/BluePrints/Stage/BP_Wing_Bird.BP_Wing_Bird_C|Getmissed _asbp_wing_bird)
    (Variables|Default|Setフラグ-ポーズできない true) ; ポーズができないようにする
    (CallFunction|ポーズを解除してメニューを閉じる)
    ;[1 1 1] ゲームオーバーアニメーションを再生する
    (Utilities|FlowControl|DoOnce false
      (:Completed
        (Audio|PlaySound2D "/Game/Sound/SE/失格（カーン・・・）_Cue.失格（カーン・・・）_Cue" 1.0 1.0 0.0 0 0)
        (Audio|Components|Audio|FadeOut (Variables|Default|GetBGM) 1.0 0.0 "Linear" :!class /Script/Engine.AudioComponent)
        (UserInterface|Viewport|AddtoViewport _miss_value 0)
        (bind _asumg_game_miss (Utilities|Casting|CastToWBP_Game_Miss _miss_value)
          (:then
            _)
          (:CastFailed
            _))
        (Components|Animation|PlayAnimation _asumg_game_miss (Variables|/Game/BluePrints/WidgetBluePrint/WBP_Game_Miss.WBP_Game_Miss_C|GetIN _asumg_game_miss) 0.0
          (:then
            (Variables|Default|Setフラグ-アニメ再生中ならばストップ true))
          (:Finished
            (UserInterface|Animation|PlayAnimation _asumg_game_miss (Variables|/Game/BluePrints/WidgetBluePrint/WBP_Game_Miss.WBP_Game_Miss_C|Get点滅 _asumg_game_miss) 0.0 0 "Forward" 1.0 false)
            (Variables|Default|Setフラグ-ミス画面を出している true)
            (Variables|Default|Setフラグ-アニメ再生中ならばストップ false)))))
    (else
      ;[1 1 1] ゴールしたか?
      (bind _result (Default|GetIsGoal _asbp_wing_bird))
      (if _result
        ;[1 1 1] ゴール画面を再生する
        (Utilities|FlowControl|DoOnce false
          (:Completed
            (Variables|Default|Setフラグ-ゴールした true)
            (Audio|Components|Audio|FadeOut (Variables|Default|GetBGM) 0.0 0.0 "Linear" :!class /Script/Engine.AudioComponent)
            (CallFunction|SE-ゴール)
            (Variables|Default|Setフラグ-ポーズできない true)
            (CallFunction|ポーズを解除してメニューを閉じる)
            (Variables|Default|Setフラグ-アニメ再生中ならばストップ true)
            (Utilities|FlowControl|Delay 1.5)
            (UserInterface|Viewport|AddtoViewport _goal_value 0)
            (bind _asumg_game_clear (Utilities|Casting|CastToWBP_Game_Clear _goal_value)
              (:then
                _)
              (:CastFailed
                _))
            (UserInterface|Animation|PlayAnimation _asumg_game_clear (Variables|/Game/BluePrints/WidgetBluePrint/WBP_Game_Clear.WBP_Game_Clear_C|Get点滅 _asumg_game_clear) 0.0 0 "Forward" 1.0 false)
            (Variables|Default|Setフラグ-アニメ再生中ならばストップ false)
            (Utilities|FlowControl|Delay 0.5)
            (bind _returnvalue (Audio|CreateSound2D "/Game/Sound/BGM/StageClear.StageClear" 1.0 1.0 0.0 0))
            (Audio|Components|Audio|Play _returnvalue 0.0)))))))

(event EventBeginPlay
  ;[1 1 1] BGM
  (bind _returnvalue (Game|GetCurrentLevelName true))
  (bind _returnvalue_2 (Utilities|GetDataTableRow "/Game/BluePrints/DT_Stage_List.DT_Stage_List" (Utilities|String|StringToName _returnvalue))
    (:then
      (switch int (.BGM (Utilities|Struct|BreakStruct_StageLevelData _returnvalue_2))
        (:Default
          (bind _returnvalue_3 (Audio|CreateSound2D "/Game/Sound/BGM/Stage1BGM.Stage1BGM" 1.0 1.0 0.0 0 :!label _label))
          (Variables|Default|SetBGM _returnvalue_3))
        (:0
          (goto _label))
        (:1
          (bind _returnvalue_4 (Audio|CreateSound2D "/Game/Sound/BGM/Stage2BGM.Stage2BGM" 1.0 1.0 0.0 0))
          (Variables|Default|SetBGM _returnvalue_4))
        (:2
          (bind _returnvalue_5 (Audio|CreateSound2D "/Game/Sound/BGM/Stage3BGM.Stage3BGM" 1.0 1.0 0.0 0))
          (Variables|Default|SetBGM _returnvalue_5))
        (:3
          (goto _label))))
    (:RowNotFound
      _))
  (Audio|Components|Audio|Play (Variables|Default|GetBGM) 0.0)
  ;[1 1 1] ポーズ画面を作っておく
  (bind _returnvalue_6 (UserInterface|CreateWidget (Variables|Default|Getpause%20menu)))
  (Variables|Default|Setpause_menu_value _returnvalue_6)
  ;[1 1 1] フラグをセットする
  (Variables|Default|Setフラグ-ポーズできない true)
  (Variables|Default|Setフラグ-ミス画面を出している false)
  (Variables|Default|Setフラグ-スタートしたか? false)
  ;[1 1 1] ミス画面を作っておく
  (bind _returnvalue_7 (UserInterface|CreateWidget (Variables|Default|Getmiss)))
  (Variables|Default|Setmiss_value _returnvalue_7)
  ;[1 1 1] ゴール画面を作っておく
  (bind _returnvalue_8 (UserInterface|CreateWidget (Variables|Default|GetGoal)))
  (Variables|Default|SetGoal_value _returnvalue_8)
  ;[1 1 1] コメント
  (bind _returnvalue_9 (UserInterface|CreateWidget (Variables|Default|GetGame_State)))
  (UserInterface|Viewport|AddtoViewport _returnvalue_9 -1)
  ;[1 1 1] ゲームのスタート画面を作りセットする
  (bind _returnvalue_10 (UserInterface|CreateWidget (Variables|Default|GetStart%20widget)))
  (UserInterface|Viewport|AddtoViewport _returnvalue_10 10)
  (bind _output_get (Variables|Default|Setstart%20widget%20value _returnvalue_10))
  (bind _asumg_game_start (Utilities|Casting|CastToWBP_Game_Start _output_get)
    (:then
      _)
    (:CastFailed
      _))
  (Components|Animation|PlayAnimation _output_get (Variables|/Game/BluePrints/WidgetBluePrint/WBP_Game_Start.WBP_Game_Start_C|GetFadeIn _asumg_game_start) 0.0
    (:then
      (Variables|Default|Setフラグ-アニメ再生中ならばストップ true))
    (:Finished
      (UserInterface|Animation|PlayAnimation _output_get (Variables|/Game/BluePrints/WidgetBluePrint/WBP_Game_Start.WBP_Game_Start_C|Gettenmetu _asumg_game_start) 0.0 0 "Forward" 1.0 true)
      (Variables|Default|Setフラグ-アニメ再生中ならばストップ false))))

(event Input|ActionEvents|InputActionメニューボタン
  (params (Key :type Key%20Structure))
  (:Pressed
    (if (not (Variables|Default|Getフラグ-ポーズできない))
      (if (not (Variables|Default|Getフラグ-ミス画面を出している))
        (if (not (Variables|Default|Getフラグ-アニメ再生中ならばストップ))
          (Audio|PlaySound2D "/Game/Sound/SE/メニュー開く_Cue.メニュー開く_Cue" 1.0 1.0 0.0 0 0)
          (if (Game|IsGamePaused)
            (CallFunction|ポーズを解除してメニューを閉じる)
            (else
              (CallFunction|ゲームをポーズにしてメニューを開く))))))))

(event Input|ActionEvents|InputAction決定ボタン
  (params (Key :type Key%20Structure))
  (bind _start_widget_value (Variables|Default|Getstart%20widget%20value))
  (bind _start_widget_value_2 (Variables|Default|Getstart%20widget%20value))
  (:Pressed
    (if (not (Variables|Default|Getフラグ-アニメ再生中ならばストップ))
      (if (not (Variables|Default|Getフラグ-スタートしたか?))
        ;[1 1 1] 鳥の変数をいじって動き出させる
        (bind _asbp_wing_bird (Utilities|Casting|CastToBP_Wing_Bird (Pawn|GetControlledPawn))
          (:then
            _)
          (:CastFailed
            _))
        (Variables|/Game/BluePrints/Stage/BP_Wing_Bird.BP_Wing_Bird_C|Setalready_started _asbp_wing_bird true)
        ;[1 1 1] 各種フラグを変更する
        (Variables|Default|Setフラグ-スタートしたか? true) ; スタートした
        (Variables|Default|Setフラグ-ポーズできない false) ; ポーズ不可解除
        (Widget|RemovefromParent (Variables|Default|Getstart%20widget%20value))
        (CallFunction|SE-スタート)
        (elif (Variables|Default|Getフラグ-ゴールした)
          ;[1 1 1] ゴール画面の処理
          (bind _asumg_game_clear (Utilities|Casting|CastToWBP_Game_Clear (Variables|Default|GetGoal_value))
            (:then
              _)
            (:CastFailed
              _))
          (Components|Animation|PlayAnimation _asumg_game_clear (Variables|/Game/BluePrints/WidgetBluePrint/WBP_Game_Clear.WBP_Game_Clear_C|GetOUT _asumg_game_clear) 0.0
            (:then
              (Variables|Default|Setフラグ-アニメ再生中ならばストップ true)
              (CallFunction|SE-決定)
              ;;[1 1 1] Save処理
              (bind _asbp_my_game_instance (Utilities|Casting|CastToBP_My_Game_Instance (Game|GetGameInstance)))
              (bind _returnvalue (Game|GetCurrentLevelName true))
              (bind _returnvalue_2 (Utilities|GetDataTableRow "/Game/BluePrints/DT_Stage_List.DT_Stage_List" (Utilities|String|StringToName _returnvalue))
                (:then
                  (bind _asbp_my_player_state (Utilities|Casting|CastToBP_My_Player_State (Game|GetPlayerState 0)))
                  (Default|Save-Stageクリア _asbp_my_game_instance (.StageNum (Utilities|Struct|BreakStruct_StageLevelData _returnvalue_2)) (Variables|/Game/BluePrints/Stage/BP_My_Player_State.BP_My_Player_State_C|Getハート取得済み1 _asbp_my_player_state) (Variables|/Game/BluePrints/Stage/BP_My_Player_State.BP_My_Player_State_C|Getハート取得済み2 _asbp_my_player_state) (Variables|/Game/BluePrints/Stage/BP_My_Player_State.BP_My_Player_State_C|Getハート取得済み3 _asbp_my_player_state)))))
            (:Finished
              (CallFunction|ステージ選択に戻る)))
          (elif (Variables|Default|Getフラグ-ミス画面を出している)
            ;[1 1 1] ミス画面の処理
            (bind _asumg_game_miss (Utilities|Casting|CastToWBP_Game_Miss (Variables|Default|Getmiss_value))
              (:then
                _)
              (:CastFailed
                _))
            (Components|Animation|PlayAnimation _asumg_game_miss (Variables|/Game/BluePrints/WidgetBluePrint/WBP_Game_Miss.WBP_Game_Miss_C|GetOUT _asumg_game_miss) 0.0
              (:then
                (Variables|Default|Setフラグ-アニメ再生中ならばストップ true)
                (CallFunction|SE-決定))
              (:Finished
                (CallFunction|ステージを開きなおす)))
            (elif (Game|IsGamePaused) ; ゲームがポーズ中，つまりメニューを開いているときのみ
              ;[1 1 1] メニュー画面の処理
              (CallFunction|SE-決定)
              (switch int (Math|Integer|%(Integer) (Variables|Default|Getメニューのどれを選択しているか) (Variables|Default|Getメニューの数))
                (:Default
                  (Development|PrintText "メニュー選択でおかしな値が選択されました") ; ふつうは実行されない
                )
                (:0
                  (CallFunction|ポーズを解除してメニューを閉じる) ; 再開の処理
                )
                (:1
                  (UserInterface|Viewport|AddtoViewport _start_widget_value_2 0)
                  (bind _asumg_game_start (Utilities|Casting|CastToWBP_Game_Start _start_widget_value_2)
                    (:then
                      _)
                    (:CastFailed
                      _))
                  (UserInterface|Animation|PlayAnimation _asumg_game_start (Variables|/Game/BluePrints/WidgetBluePrint/WBP_Game_Start.WBP_Game_Start_C|GetFadeIn _asumg_game_start) 0.0 1 "Reverse" 1.0 false)
                  (Variables|Default|Setフラグ-アニメ再生中ならばストップ true)
                  (Utilities|FlowControl|Delay 1.0)
                  (CallFunction|ステージを開きなおす) ; スタートに戻る
                )
                (:2
                  (UserInterface|Viewport|AddtoViewport _start_widget_value 0)
                  (bind _asumg_game_start_2 (Utilities|Casting|CastToWBP_Game_Start _start_widget_value)
                    (:then
                      _)
                    (:CastFailed
                      _))
                  (UserInterface|Animation|PlayAnimation _asumg_game_start_2 (Variables|/Game/BluePrints/WidgetBluePrint/WBP_Game_Start.WBP_Game_Start_C|GetFadeIn _asumg_game_start_2) 0.0 1 "Reverse" 1.0 false)
                  (Variables|Default|Setフラグ-アニメ再生中ならばストップ true)
                  (Utilities|FlowControl|Delay 1.0)
                  (CallFunction|ステージ選択に戻る))))))))))

(event Input|ActionEvents|InputActionメニュー下ボタン
  (params (Key :type Key%20Structure))
  (:Pressed
    (if (not (Variables|Default|Getフラグ-アニメ再生中ならばストップ))
      (if (Game|IsGamePaused) ; ゲームがポーズ中，つまりメニューを開いているときのみ
        ;[1 1 1] メニュー画面が開かれているならば実行する
        (CallFunction|下にメニューを移してアニメーションする)
        (CallFunction|SE-選択変更)))))

(event Input|ActionEvents|InputActionメニュー上ボタン
  (params (Key :type Key%20Structure))
  (:Pressed
    (if (not (Variables|Default|Getフラグ-アニメ再生中ならばストップ))
      (if (Game|IsGamePaused) ; ゲームがポーズ中，つまりメニューを開いているときのみ
        ;[1 1 1] メニュー画面が開かれているならば実行する
        (CallFunction|上にメニューを移してアニメーションする)
        (CallFunction|SE-選択変更)))))

(fn ConstructionScript)

(fn ゲームをポーズにしてメニューを開く
  (bind _pause_menu_value (Variables|Default|Getpause_menu_value))
  (UserInterface|Viewport|AddtoViewport _pause_menu_value 0) ; メニューを画面に追加
  (bind _asumg_game_pause (Utilities|Casting|CastToWBP_Game_Pause _pause_menu_value) ; アニメーションを取得するためにキャスト
    (:then
      _)
    (:CastFailed
      _))
  (UserInterface|Animation|PlayAnimation _asumg_game_pause (Variables|/Game/BluePrints/WidgetBluePrint/WBP_Game_Pause.WBP_Game_Pause_C|Get再開を選択中 _asumg_game_pause) 0.0 1 "Forward" 1.0 false) ; アニメーション再生
  (Variables|Default|Setメニューのどれを選択しているか 0) ; 再開に合わせる
  (Game|SetGamePaused true))

(fn ポーズを解除してメニューを閉じる
  (Widget|RemovefromParent (Variables|Default|Getpause_menu_value))
  (Game|SetGamePaused false))

(fn ステージを開きなおす
  (bind _returnvalue (Game|GetCurrentLevelName true))
  (Game|OpenLevel(byName) (Utilities|String|StringToName _returnvalue)))

(fn 上にメニューを移してアニメーションする
  (bind _pause_menu_value (Variables|Default|Getpause_menu_value))
  (Variables|Default|Setメニューのどれを選択しているか (+ (Variables|Default|Getメニューのどれを選択しているか) 2))
  (Class|UserWidget|StopAllAnimations (Variables|Default|Getpause_menu_value))
  (switch int (Math|Integer|%(Integer) (Variables|Default|Getメニューのどれを選択しているか) (Variables|Default|Getメニューの数))
    (:0
      (bind _asumg_game_pause (Utilities|Casting|CastToWBP_Game_Pause _pause_menu_value)
        (:then
          _)
        (:CastFailed
          _))
      (UserInterface|Animation|PlayAnimation _pause_menu_value (Variables|/Game/BluePrints/WidgetBluePrint/WBP_Game_Pause.WBP_Game_Pause_C|Get再開を選択中 _asumg_game_pause) 0.0 1 "Forward" 1.0 true))
    (:1
      (bind _asumg_game_pause_2 (Utilities|Casting|CastToWBP_Game_Pause _pause_menu_value)
        (:then
          _)
        (:CastFailed
          _))
      (UserInterface|Animation|PlayAnimation _pause_menu_value (Variables|/Game/BluePrints/WidgetBluePrint/WBP_Game_Pause.WBP_Game_Pause_C|Getスタートを選択中 _asumg_game_pause_2) 0.0 1 "Forward" 1.0 true))
    (:2
      (bind _asumg_game_pause_3 (Utilities|Casting|CastToWBP_Game_Pause _pause_menu_value)
        (:then
          _)
        (:CastFailed
          _))
      (UserInterface|Animation|PlayAnimation _pause_menu_value (Variables|/Game/BluePrints/WidgetBluePrint/WBP_Game_Pause.WBP_Game_Pause_C|Getステージ選択を選択中 _asumg_game_pause_3) 0.0 1 "Forward" 1.0 true))))

(fn 下にメニューを移してアニメーションする
  (bind _pause_menu_value (Variables|Default|Getpause_menu_value))
  (Variables|Default|Setメニューのどれを選択しているか (+ (Variables|Default|Getメニューのどれを選択しているか) 1))
  (Class|UserWidget|StopAllAnimations (Variables|Default|Getpause_menu_value))
  (switch int (Math|Integer|%(Integer) (Variables|Default|Getメニューのどれを選択しているか) (Variables|Default|Getメニューの数))
    (:0
      (bind _asumg_game_pause (Utilities|Casting|CastToWBP_Game_Pause _pause_menu_value)
        (:then
          _)
        (:CastFailed
          _))
      (UserInterface|Animation|PlayAnimation _pause_menu_value (Variables|/Game/BluePrints/WidgetBluePrint/WBP_Game_Pause.WBP_Game_Pause_C|Get再開を選択中 _asumg_game_pause) 0.0 1 "Forward" 1.0 true))
    (:1
      (bind _asumg_game_pause_2 (Utilities|Casting|CastToWBP_Game_Pause _pause_menu_value)
        (:then
          _)
        (:CastFailed
          _))
      (UserInterface|Animation|PlayAnimation _pause_menu_value (Variables|/Game/BluePrints/WidgetBluePrint/WBP_Game_Pause.WBP_Game_Pause_C|Getスタートを選択中 _asumg_game_pause_2) 0.0 1 "Forward" 1.0 true))
    (:2
      (bind _asumg_game_pause_3 (Utilities|Casting|CastToWBP_Game_Pause _pause_menu_value)
        (:then
          _)
        (:CastFailed
          _))
      (UserInterface|Animation|PlayAnimation _pause_menu_value (Variables|/Game/BluePrints/WidgetBluePrint/WBP_Game_Pause.WBP_Game_Pause_C|Getステージ選択を選択中 _asumg_game_pause_3) 0.0 1 "Forward" 1.0 true))))

(fn ステージ選択に戻る
  (Game|OpenLevel(byObjectReference) "/Game/Levels/StageSelect.StageSelect"))

(fn SE-選択変更
  (Audio|PlaySound2D "/Game/Sound/SE/魔王魂_効果音_システム21_Cue.魔王魂_効果音_システム21_Cue" 1.0 1.0 0.0 0 0))

(fn SE-決定
  (Audio|PlaySound2D "/Game/Sound/SE/魔王魂_効果音_システム46_Cue.魔王魂_効果音_システム46_Cue" 1.0 1.0 0.0 0 0))

(fn SE-ゴール
  (Audio|PlaySound2D "/Game/Sound/SE/ゴールした.ゴールした" 1.0 1.0 0.0 0 0))

(fn SE-スタート
  (Audio|PlaySound2D "/Game/Sound/SE/スタートした.スタートした" 1.0 1.0 0.0 0 0))