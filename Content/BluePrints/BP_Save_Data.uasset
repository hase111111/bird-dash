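; BP_Save_Data holds per-stage clear data: a cleared flag and three heart flags for each stage.
; The stage-clear function ORs new heart results with stored ones, so earned hearts persist, then marks the stage cleared.
; It also range-checks the stage number, printing an overflow warning when invalid.
; A getter totals the hearts earned across all stages.
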(fn ステージクリア
  (params (stagenum :type Integer) (h1 :type Boolean) (h2 :type Boolean) (h3 :type Boolean))
  (bind _stage_data (Variables|Default|GetStage_Data))
  (bind _output (Utilities|Array|Get(acopy) _stage_data stagenum))
  (if (Math|Integer|InRange(Integer) stagenum 0 15)
    _
    (else
      (Development|PrintString 0 "オーバーフロー対策で実行しません")))
  (if (or h1 (.ハート1 _output))
    (Variables|Default|Settemp1 true)
    (else
      (Variables|Default|Settemp1 false)))
  (if (or h2 (.ハート2 _output))
    (Variables|Default|Settemp2 true)
    (else
      (Variables|Default|Settemp2 false)))
  (if (or h3 (.ハート3 _output))
    (Variables|Default|Settemp3 true)
    (else
      (Variables|Default|Settemp3 false)))
  (Utilities|Array|SetArrayElem (Variables|Default|GetStage_Data) stagenum (Utilities|Struct|MakeStruct_1Stage_ClearData (Variables|Default|Gettemp1) (Variables|Default|Gettemp2) (Variables|Default|Gettemp3) true)))

(fn Get全ハート数
  (Variables|Default|Settemp 0)
  (for _array_element (Variables|Default|GetStage_Data)
    (if (.ハート1 (Utilities|Struct|BreakStruct_1Stage_ClearData _array_element))
      (Variables|Default|Settemp (+ (Variables|Default|Gettemp) 1)))
    (if (.ハート2 (Utilities|Struct|BreakStruct_1Stage_ClearData _array_element))
      (Variables|Default|Settemp (+ (Variables|Default|Gettemp) 1)))
    (if (.ハート3 (Utilities|Struct|BreakStruct_1Stage_ClearData _array_element))
      (Variables|Default|Settemp (+ (Variables|Default|Gettemp) 1))))
  (return (Variables|Default|Gettemp)))