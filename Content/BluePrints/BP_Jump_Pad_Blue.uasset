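; Blue jump pad actor that pops away from its spot when the player first touches it.
; A tagged player overlapping the mesh fires a DoOnce that starts the motion, seeds vertical velocity and replaces the pad's Tags with EmptyTag.
; Tick then applies hand-rolled, per-frame kinematics without delta time or sweep, adding acceleration to Z movement while spinning the pad in pitch.
; The player's bounce is not handled here.
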(event OnComponentBeginOverlap(StaticMesh)
  (params (OverlappedComponent :type Primitive%20Component%20Object%20Reference) (OtherActor :type Actor%20Object%20Reference) (OtherComp :type Primitive%20Component%20Object%20Reference) (OtherBodyIndex :type Integer) (bFromSweep :type Boolean) (SweepResult :type Hit%20Result%20Structure%20%28by%20ref%29))
  (Utilities|IsValid OtherActor
    (:Is%20Valid
      (if (Actor|ActorHasTag OtherActor (Variables|Default|Getplayer_tag)) ; ヒットしたら
        (Utilities|FlowControl|DoOnce false
          (:Completed
            (Variables|Default|Setstarted_physics_calc true)
            (Variables|Default|Setvec_z 8.0)
            (Variables|Default|SetTags (Variables|Default|Getempty_tag))))))))

(event EventTick
  (params (DeltaSeconds :type Float%20%28single-precision%29))
  (bind _returnvalue (Transformation|GetActorRotation))
  (bind _returnvalue_2 (Transformation|GetActorLocation))
  (if (Variables|Default|Getstarted_physics_calc)
    (Variables|Default|Setvec_z (+ (Variables|Default|Getvec_z) (Variables|Default|Getacc_z)))
    (Transformation|SetActorLocation (Math|Vector|MakeVector (.x _returnvalue_2) (.y _returnvalue_2) (+ (.z _returnvalue_2) (Variables|Default|Getvec_z))) false false)
    (bind _output_get (Variables|Default|Setrot_value (Math|Rotator|MakeRotator (.roll _returnvalue) (+ (.pitch _returnvalue) (Variables|Default|Getrot_speed)) (.yaw _returnvalue))))
    (Transformation|SetActorRotation _output_get)))

(fn ConstructionScript)