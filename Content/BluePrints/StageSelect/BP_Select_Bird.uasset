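; BP_Select_Bird is the stage select bird that glides along the Y axis to the chosen stage.
; A setter function stores the destination index, which Tick uses to look up a Y coordinate and interpolate the actor there with VInterpTo while it is in range.
; Tick also compares Y with the previous frame's position to flip the mesh toward the direction of travel using fast RInterpTo.
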(event EventTick
  (params (DeltaSeconds :type Float%20%28single-precision%29))
  (bind _mesh (Variables|Character|GetMesh))
  (if (Math|Integer|InRange(Integer) (Variables|Default|Getステージの移動先) 0 15)
    (Transformation|SetActorLocation (Math|Interpolation|VInterpTo (Transformation|GetActorLocation) (Math|Vector|MakeVector 0.0 (Utilities|Array|Get(acopy) (Variables|Default|GetStageのy座標) (Variables|Default|Getステージの移動先)) 0.0) (Utilities|Time|GetWorldDeltaSeconds) 5.0) false true))
  ;[1 1 1] 向きを決める
  (if (>= (.y (Transformation|GetActorLocation)) (.y (Variables|Default|Get向きを決めるために使う座標)))
    (Transformation|SetRelativeRotation _mesh (Math|Interpolation|RInterpTo (Transformation|GetActorRotation) "0, 0, 0" (Utilities|Time|GetWorldDeltaSeconds) 1e+02) false false)
    (else
      (Transformation|SetRelativeRotation _mesh (Math|Interpolation|RInterpTo (Transformation|GetActorRotation) "0,180.000000, 0" (Utilities|Time|GetWorldDeltaSeconds) 1e+02) false false)))
  (Variables|Default|Set向きを決めるために使う座標 (Transformation|GetActorLocation)))

(fn ConstructionScript)

(fn ステージの移動先をセットする
  (params (NewParam :type Integer))
  (Variables|Default|Setステージの移動先 NewParam))