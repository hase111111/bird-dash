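; BP_Player_Camera is a camera actor that follows the player, normally BP_Bird_Wing, each Tick.
; It sits behind along Y at a height offset and aims ahead of the player, capping the look target's Z at zero.
; The bird's goal flag stops the Y follow for a finish shot while X, Z and aim keep tracking; its collision flag freezes the camera.
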(event EventTick
  (params (DeltaSeconds :type Float%20%28single-precision%29))
  (bind _returnvalue (Game|GetPlayerCharacter 0))
  (bind _returnvalue_2 (Transformation|GetActorLocation _returnvalue))
  (bind _returnvalue_3 (Transformation|GetActorLocation _returnvalue))
  (bind _returnvalue_4 (Transformation|GetActorLocation _returnvalue))
  (Utilities|IsValid _returnvalue
    (:Is%20Valid
      (bind _asbp_bird_wing (Utilities|Casting|CastToBP_Bird_Wing _returnvalue)
        (:then
          (bind _result (Default|Getフラグゴールした _asbp_bird_wing))
          (if _result
            ;[1 1 1] ゴール演出
            (Transformation|SetActorLocation (Math|Vector|MakeVector (.x _returnvalue_4) (.y (Transformation|GetActorLocation)) (+ (.z _returnvalue_4) (Variables|Default|Get高さの座標))) false true)
            ;[1 1 1] カメラの向きセット
            (Transformation|SetActorRotation (Math|Rotator|FindLookatRotation (Transformation|GetActorLocation) (Math|Vector|MakeVector (.x _returnvalue_2) (+ (.y _returnvalue_2) (Variables|Default|Getプレイヤーより前に行く)) (Variables|Default|GetZ))) true :!label _label)
            (else
              (bind _result_2 (Default|Getフラグ衝突した _asbp_bird_wing))
              (if (not _result_2)
                ;[1 1 1] カメラの位置セット
                (Transformation|SetActorLocation (Math|Vector|MakeVector (.x _returnvalue_3) (- (.y _returnvalue_3) (Variables|Default|Getどのくらい後ろか)) (+ (.z _returnvalue_3) (Variables|Default|Get高さの座標))) false true :!label _label_2)
                (if (< (.z _returnvalue_2) 0.0)
                  (Variables|Default|SetZ (.z _returnvalue_2))
                  (goto _label)
                  (else
                    (Variables|Default|SetZ 0.0)
                    (goto _label)))))))
        (:CastFailed
          (goto _label_2))))))

(fn ConstructionScript)