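; BP_Obstacle_Log is a log obstacle that starts rolling along negative Y when the player gets close.
; Tick compares the player's Y position with the log's, offset by a reaction-distance variable, then latches a movement flag and starts a ten-second lifespan.
; Once triggered, it adds fixed roll and location steps every frame without sweep or delta-time scaling.
; BeginPlay sets the actor's tags from a variable.
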(event EventBeginPlay
  (Variables|Default|SetTags (Variables|Default|GetTags_0)))

(event EventTick
  (params (DeltaSeconds :type Float%20%28single-precision%29))
  (bind _returnvalue (Transformation|GetActorLocation))
  (if (Variables|Default|Get移動開始)
    (Transformation|SetActorRotation (Math|Rotator|MakeRotator (+ (.roll (Transformation|GetActorRotation)) -3.0) 0.0 0.0))
    (Transformation|SetActorLocation (Math|Vector|MakeVector (.x _returnvalue) (+ (.y _returnvalue) -5.0) (.z _returnvalue)) false false)
    (elif (> (.y (Transformation|GetActorLocation (Game|GetPlayerCharacter 0))) (- (.y (Transformation|GetActorLocation)) (Variables|Default|Getどの程度で反応するかどうか)))
      (Variables|Default|Set移動開始 true)
      (Actor|SetLifeSpan 1e+01))))

(fn ConstructionScript)