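; BP_Blinde_Lift is a triggered moving mesh that drops from a raised position when the player arrives.
; BeginPlay raises the mesh and disables Tick; a player-tagged actor entering the Box re-enables Tick and plays a machinery sound once.
; Tick lowers ZPos by a fixed, frame-rate-dependent step, then snaps the mesh to its relative origin and switches Tick off again.
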(event OnComponentBeginOverlap(Box)
  (params (OverlappedComponent :type Primitive%20Component%20Object%20Reference) (OtherActor :type Actor%20Object%20Reference) (OtherComp :type Primitive%20Component%20Object%20Reference) (OtherBodyIndex :type Integer) (bFromSweep :type Boolean) (SweepResult :type Hit%20Result%20Structure%20%28by%20ref%29))
  (Utilities|IsValid OtherActor
    (:Is%20Valid
      (if (Actor|ActorHasTag OtherActor "player")
        (Actor|Tick|SetActorTickEnabled true)
        (Utilities|FlowControl|DoOnce false
          (:Completed
            (Audio|PlaySound2D "/Game/Sound/SE/機械音.機械音" 1.0 1.0 0.0 0 0)))))))

(event EventBeginPlay
  (Transformation|SetRelativeLocation (Variables|Default|GetStaticMesh) "0, 0,1000.000000" false false)
  (Actor|Tick|SetActorTickEnabled false))

(event EventTick
  (params (DeltaSeconds :type Float%20%28single-precision%29))
  (bind _staticmesh (Variables|Default|GetStaticMesh))
  (Variables|Default|Setz_pos (- (Variables|Default|Getz_pos) 75.0))
  (if (<= (Variables|Default|Getz_pos) 0.0)
    (Transformation|SetRelativeLocation _staticmesh "0, 0, 0" false false)
    (Actor|Tick|SetActorTickEnabled false)
    (else
      (Transformation|SetRelativeLocation _staticmesh (Math|Vector|MakeVector 0.0 0.0 (Variables|Default|Getz_pos)) false false))))

(fn ConstructionScript)