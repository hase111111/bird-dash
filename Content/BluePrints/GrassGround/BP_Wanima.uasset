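; BP_Wanima is an obstacle actor that starts moving along negative Y once the player gets close on that axis.
; BeginPlay sets its tags from ObstacleTag.
; Tick latches IsMoved when the player's Y exceeds the actor's Y minus MoveDistance, then shifts the actor a fixed step every frame.
; The movement is not scaled by delta time, does not sweep and never stops.
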(event EventBeginPlay
  (Variables|Default|SetTags (Variables|Default|Getobstacle_tag)))

(event EventTick
  (params (DeltaSeconds :type Float%20%28single-precision%29))
  (bind _returnvalue (Transformation|GetActorLocation))
  (if (Variables|Default|Getis_moved)
    (Transformation|SetActorLocation (Math|Vector|MakeVector (.x _returnvalue) (+ (.y _returnvalue) -2.5) (.z _returnvalue)) false false)
    (elif (> (.y (Transformation|GetActorLocation (Game|GetPlayerCharacter 0))) (- (.y (Transformation|GetActorLocation)) (Variables|Default|Getmove_distance)))
      (Variables|Default|Setis_moved true))))

(fn ConstructionScript)