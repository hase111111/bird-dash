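; Ostrich enemy for the GrassGround area that tags itself as an obstacle and runs along negative Y toward the oncoming player.
; Each Tick, if recently rendered and the player is within MoveDistance on Y, it shifts a fixed step without sweep, so speed depends on frame rate.
; It destroys itself once the player has passed it by a margin.
; An AddMovementInput call is left unconnected.
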(event EventBeginPlay
  ;[1 1 1] 障害物タグをつける
  (Variables|Default|SetTags (Variables|Default|Getobstacle_tag)))

(event EventTick
  (params (DeltaSeconds :type Float%20%28single-precision%29))
  (bind _returnvalue (Transformation|GetActorLocation))
  (if (Class|Actor|WasRecentlyRendered 0.2)
    (if (> (.y (Transformation|GetActorLocation (Game|GetPlayerCharacter 0))) (- (.y (Transformation|GetActorLocation)) (Variables|Default|Getmove_distance)))
      (Transformation|SetActorLocation (Math|Vector|MakeVector (.x _returnvalue) (+ (.y _returnvalue) -5.0) (.z _returnvalue)) false false)
      ;[1 1 1] プレイヤーに追い抜かれたら消える
      (if (< (+ (.y (Transformation|GetActorLocation)) 3e+02) (.y (Transformation|GetActorLocation (Game|GetPlayerCharacter 0))))
        (Actor|DestroyActor)))))

(fn ConstructionScript)