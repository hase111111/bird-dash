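; Game Instance that owns the game's save data and shares config, stage progress and the stage-select choice with the rest of the game.
; It loads or creates a BP_Save_Data slot, recreating it in most accessors if invalid, and saves on config changes and stage clears.
; Saved config drives resolution, window mode, quality, frame limit and sound-class volumes.
; Stage hearts, clear state and distance are read from a flattened 4×4 array.
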(fn セーブデータ読込，初期化処理
  (bind _returnvalue (SaveGame|DoesSaveGameExist (Variables|Default|GetSlot%20Name) (Variables|Default|GetUser%20Index)))
  ;[1 1 1] セーブデータがないなら作る
  (if _returnvalue
    ;[1 1 1] あるなら読む
    (bind _returnvalue_2 (SaveGame|LoadGamefromSlot (Variables|Default|GetSlot%20Name) (Variables|Default|GetUser%20Index)))
    (bind _asbp_save_data (Utilities|Casting|CastToBP_Save_Data _returnvalue_2))
    (Variables|Default|SetSaveData _asbp_save_data)
    (else
      (CallFunction|セーブデータ作成，保存))))

(fn セーブデータ作成，保存
  (bind _returnvalue (SaveGame|CreateSaveGameObject "/Game/BluePrints/BP_Save_Data.BP_Save_Data_C"))
  (bind _output_get (Variables|Default|SetSaveData _returnvalue))
  (Variables|/Game/BluePrints/BP_Save_Data.BP_Save_Data_C|Setconfig_data _output_get (Variables|Default|GetConfig%20Data初期値))
  (SaveGame|SaveGametoSlot _output_get (Variables|Default|GetSlot%20Name) (Variables|Default|GetUser%20Index)))

(fn コンフィグを読み，適用
  (bind _savedata (Variables|Default|GetSaveData))
  (bind _savedata_2 (Variables|Default|GetSaveData))
  (bind _config_data (Variables|/Game/BluePrints/BP_Save_Data.BP_Save_Data_C|Getconfig_data _savedata))
  (bind _config_data_2 (Variables|/Game/BluePrints/BP_Save_Data.BP_Save_Data_C|Getconfig_data _savedata_2))
  (Utilities|IsValid _savedata_2
    (:Is%20Valid
      ;[1 1 1] 解像度設定，スクリーンも
      (switch int (Math|Integer|%(Integer) (.解像度 _config_data_2) 4)
        (:Default
          (bind _returnvalue (Settings|GetGameUserSettings :!label _label))
          (Class|GameUserSettings|SetScreenResolution _returnvalue (Utilities|Struct|MakeIntPoint 960 540)))
        (:0
          (bind _returnvalue_2 (Settings|GetGameUserSettings))
          (Class|GameUserSettings|SetScreenResolution _returnvalue_2 (Utilities|Struct|MakeIntPoint 1920 1080)))
        (:1
          (bind _returnvalue_3 (Settings|GetGameUserSettings))
          (Class|GameUserSettings|SetScreenResolution _returnvalue_3 (Utilities|Struct|MakeIntPoint 1600 900)))
        (:2
          (bind _returnvalue_4 (Settings|GetGameUserSettings))
          (Class|GameUserSettings|SetScreenResolution _returnvalue_4 (Utilities|Struct|MakeIntPoint 1280 720)))
        (:3
          (goto _label)))
      (if (== (Math|Integer|%(Integer) (.スクリーン _config_data_2) 2) 0)
        (bind _returnvalue_5 (Settings|GetGameUserSettings))
        (Class|GameUserSettings|SetFullscreenMode _returnvalue_5 "Fullscreen")
        (Class|GameUserSettings|ApplySettings _returnvalue_5 false)
        (else
          (bind _returnvalue_6 (Settings|GetGameUserSettings))
          (Class|GameUserSettings|SetFullscreenMode _returnvalue_6 "Windowed")
          (Class|GameUserSettings|ApplySettings _returnvalue_6 false)))
      ;[1 1 1] 画質
      (switch int (Math|Integer|%(Integer) (.画質 (Variables|/Game/BluePrints/BP_Save_Data.BP_Save_Data_C|Getconfig_data (Variables|Default|GetSaveData))) 4)
        (:Default
          (bind _returnvalue_7 (Settings|GetGameUserSettings :!label _label_2))
          (Class|GameUserSettings|SetOverallScalabilityLevel _returnvalue_7)
          (Class|GameUserSettings|ApplySettings _returnvalue_7 false))
        (:0
          (goto _label_2))
        (:1
          (bind _returnvalue_8 (Settings|GetGameUserSettings))
          (Class|GameUserSettings|SetOverallScalabilityLevel _returnvalue_8 1)
          (Class|GameUserSettings|ApplySettings _returnvalue_8 false))
        (:2
          (bind _returnvalue_9 (Settings|GetGameUserSettings))
          (Class|GameUserSettings|SetOverallScalabilityLevel _returnvalue_9 2)
          (Class|GameUserSettings|ApplySettings _returnvalue_9 false))
        (:3
          (bind _returnvalue_10 (Settings|GetGameUserSettings))
          (Class|GameUserSettings|SetOverallScalabilityLevel _returnvalue_10 3)
          (Class|GameUserSettings|ApplySettings _returnvalue_10 false)))
      ;[1 1 1] コメント
      (if (== (Math|Integer|%(Integer) (.fps (Variables|/Game/BluePrints/BP_Save_Data.BP_Save_Data_C|Getconfig_data (Variables|Default|GetSaveData))) 2) 0)
        (bind _returnvalue_11 (Settings|GetGameUserSettings))
        (Class|GameUserSettings|SetFrameRateLimit _returnvalue_11 6e+01)
        (Class|GameUserSettings|ApplySettings _returnvalue_11 false)
        (else
          (bind _returnvalue_12 (Settings|GetGameUserSettings))
          (Class|GameUserSettings|SetFrameRateLimit _returnvalue_12 6e+01)
          (Class|GameUserSettings|ApplySettings _returnvalue_12 false)))
      (Audio|SetSoundMixClassOverride "/Game/Sound/BP_Sound_Mix.BP_Sound_Mix" "/Game/Sound/BP_SoundClass.BP_SoundClass" (/ (Math|Conversions|ToFloat(Integer) (.マスター音量 _config_data)) 1e+02) 1.0 1.0 true)
      (Audio|PushSoundMixModifier "/Game/Sound/BP_Sound_Mix.BP_Sound_Mix")
      (Audio|SetSoundMixClassOverride "/Game/Sound/BP_Sound_Mix.BP_Sound_Mix" "/Game/Sound/BGM.BGM" (/ (Math|Conversions|ToFloat(Integer) (.bgm _config_data)) 1e+02) 1.0 1.0 true)
      (Audio|PushSoundMixModifier "/Game/Sound/BP_Sound_Mix.BP_Sound_Mix")
      (Audio|SetSoundMixClassOverride "/Game/Sound/BP_Sound_Mix.BP_Sound_Mix" "/Game/Sound/SE.SE" (/ (Math|Conversions|ToFloat(Integer) (.se _config_data)) 1e+02) 1.0 1.0 true)
      (Audio|PushSoundMixModifier "/Game/Sound/BP_Sound_Mix.BP_Sound_Mix"))
    (:Is%20Not%20Valid
      (Development|PrintString "Hello"))))

(fn Save-コンフィグ
  (params (config :type Struct%20Save%20Config%20Structure))
  (bind _output_get (Variables|Default|SetSaveData (Variables|Default|GetSaveData)))
  (Variables|/Game/BluePrints/BP_Save_Data.BP_Save_Data_C|Setconfig_data _output_get config)
  (SaveGame|SaveGametoSlot _output_get (Variables|Default|GetSlot%20Name) (Variables|Default|GetUser%20Index))
  (return))

(fn Get-コンフィグ
  (Utilities|IsValid (Variables|Default|GetSaveData)
    (:Is%20Valid
      (return (Variables|/Game/BluePrints/BP_Save_Data.BP_Save_Data_C|Getconfig_data (Variables|Default|GetSaveData))))
    (:Is%20Not%20Valid
      (CallFunction|セーブデータ作成，保存)
      (return (Variables|Default|GetConfig%20Data初期値)))))

(fn Get-ステージデータ
  (params (StageX-.%20%200~3 :type Integer) (Stage.-X%20%200~3 :type Integer))
  (bind _returnvalue (* StageX-.%20%200~3 4))
  (bind _savedata (Variables|Default|GetSaveData))
  (bind _returnvalue_2 (+ _returnvalue Stage.-X%20%200~3))
  (bind _stage_data (Variables|/Game/BluePrints/BP_Save_Data.BP_Save_Data_C|Getstage_data _savedata))
  (bind _output (Utilities|Array|Get(acopy) _stage_data _returnvalue_2))
  (if (and (Math|Integer|InRange(Integer) StageX-.%20%200~3 0 3) (Math|Integer|InRange(Integer) Stage.-X%20%200~3 0 3))
    (Utilities|IsValid (Variables|Default|GetSaveData)
      (:Is%20Valid
        (return (.ハート1 _output) (.ハート2 _output) (.ハート3 _output) (.クリア _output) (.距離 _output)))
      (:Is%20Not%20Valid
        (CallFunction|セーブデータ作成，保存)
        (return false false false false 0.0)))
    (else
      (return false false false false 0.0))))

(fn Get-全ハート数
  (bind _savedata (Variables|Default|GetSaveData))
  (Utilities|IsValid _savedata
    (:Is%20Valid
      (bind _newparam (Default|GetAllHeartNum _savedata))
      (return _newparam))
    (:Is%20Not%20Valid
      (CallFunction|セーブデータ作成，保存)
      (return 0))))

(fn Save-Stageクリア
  (params (StageNum :type Integer) (h1 :type Boolean) (h2 :type Boolean) (h3 :type Boolean))
  (bind _savedata (Variables|Default|GetSaveData))
  (Utilities|IsValid _savedata
    (:Is%20Valid
      _)
    (:Is%20Not%20Valid
      (CallFunction|セーブデータ作成，保存)))
  (Default|StageClear _savedata StageNum h1 h2 h3)
  (SaveGame|SaveGametoSlot (Variables|Default|GetSaveData) (Variables|Default|GetSlot%20Name) (Variables|Default|GetUser%20Index)))

(fn SelectStageSet選択肢
  (params (NewParam :type Integer))
  (Variables|Default|SetSelectStageの選択肢 NewParam))

(fn SelectStageGet選択肢
  (return (Variables|Default|GetSelectStageの選択肢)))