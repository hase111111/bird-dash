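; Ostrich enemy actor, tagged as an obstacle, that moves continuously in a horizontal circle around its starting location.
; BeginPlay stores that location as the center and seeds the angle from Phase.
; Tick advances the angle by Velocity, places the actor at Radius using cosine and sine without sweeping, and sets a radial look-at rotation that points outward for non-negative Velocity and inward for negative.
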(event EventBeginPlay
  ;[1 1 1] 障害物タグをつける
  (Variables|Default|SetTags (Variables|コンポーネント|GetObstacle))
  ;[1 1 1] 回転の中心座標
  (Variables|Default|Setcenter_pos (Transformation|GetActorLocation))
  (Variables|Default|Setangle (Variables|Default|Getphase)))

(event EventTick
  (params (DeltaSeconds :type Float%20%28single-precision%29))
  (bind _center_pos (Variables|Default|Getcenter_pos))
  (bind _radius (Variables|Default|Getradius))
  (bind _output_get (Variables|Default|Setangle (+ (* DeltaSeconds (Variables|Default|Getvelocity)) (Variables|Default|Getangle))))
  (Transformation|SetActorLocation (Math|Vector|MakeVector (+ (* (Math|Trig|Cos(Degrees) _output_get) _radius) (.x _center_pos)) (+ (* (Math|Trig|Sin(Degrees) _output_get) _radius) (.y _center_pos)) (.z _center_pos)) false false)
  (if (>= (Variables|Default|Getvelocity) 0.0)
    (Transformation|SetActorRotation (Math|Rotator|FindLookatRotation (Variables|Default|Getcenter_pos) (Transformation|GetActorLocation)) true)
    (else
      (Transformation|SetActorRotation (Math|Rotator|FindLookatRotation (Transformation|GetActorLocation) (Variables|Default|Getcenter_pos)) true))))

(fn ConstructionScript)