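; Player bird character for an auto-runner stage: moves forward along +Y once started, with left/right steering and jump-pad jumps.
; Tagged overlaps and hits set goal or crash flags, which Tick uses to switch movement.
; Goal slows it and steers toward the level's DataTable goal X; crashes knock it backward before stopping.
; Falling too low hides it and flags a miss; a separate function sets speed tiers.
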(event OnComponentBeginOverlap(CapsuleComponent)
  (params (OverlappedComponent :type Primitive%20Component%20Object%20Reference) (OtherActor :type Actor%20Object%20Reference) (OtherComp :type Primitive%20Component%20Object%20Reference) (OtherBodyIndex :type Integer) (bFromSweep :type Boolean) (SweepResult :type Hit%20Result%20Structure%20%28by%20ref%29))
  ;[1 1 1] ジャンプパッドの挙動
  (Utilities|IsValid OtherActor
    (:Is%20Valid
      (if (Actor|ActorHasTag OtherActor (Variables|Default|GetTag-JumpPad))
        (Character|Jump)
        (Audio|PlaySoundatLocation "/Game/Sound/SE/ジャンプする.ジャンプする" (Transformation|GetActorLocation) "0, 0, 0" 1.0 1.0 0.0 0 0 0 0)
        (else
          ;[1 1 1] ゴール時の処理
          (if (not (Variables|Default|Getフラグ-ゴールした)) ; まだゴールしていない
            (if (Actor|ActorHasTag OtherActor (Variables|Default|GetTag-Goal))
              (Utilities|FlowControl|DoOnce false
                (:Completed
                  (Variables|Default|Setフラグ-ゴールした true))))))))))

(event OnComponentHit(CapsuleComponent)
  (params (HitComponent :type Primitive%20Component%20Object%20Reference) (OtherActor :type Actor%20Object%20Reference) (OtherComp :type Primitive%20Component%20Object%20Reference) (NormalImpulse :type Vector :default "0, 0, 0") (Hit :type Hit%20Result%20Structure%20%28by%20ref%29))
  ;[1 1 1] 障害物に当たった時の挙動
  (Utilities|IsValid OtherActor
    (:Is%20Valid
      (if (Actor|ActorHasTag OtherActor (Variables|Default|GetTag-obstacle)) ; ヒットしたら
        (if (not (Variables|Default|Getフラグ-ゴールした)) ; ゴールしてないなら
          (Utilities|FlowControl|DoOnce false
            (:Completed
              (Variables|Default|Setフラグ-衝突した true)
              (Audio|PlaySound2D "/Game/Sound/SE/ぶつかった.ぶつかった" 1.0 1.0 0.0 0 0))))))))

(event EventBeginPlay
  ;[1 1 1] プレイヤータグをつける
  (Variables|Default|SetTags (Variables|Default|GetTag-Player)))

(event EventTick
  (params (DeltaSeconds :type Float%20%28single-precision%29))
  (bind _returnvalue (Transformation|GetActorLocation))
  (bind _charactermovement (Variables|Character|GetCharacterMovement))
  (bind _ミスしたときの吹っ飛び方向 (Variables|Default|Getミスしたときの吹っ飛び方向))
  (bind _returnvalue_2 (Math|Rotator|GetRotationXVector _ミスしたときの吹っ飛び方向))
  (if (Variables|Default|Getフラグ-スタートしたか?) ; まだスタートしていないならば待機
    (if (Variables|Default|Getフラグ-ゴールした)
      ;[1 1 1] ゴール時演出
      (bind _returnvalue_3 (Game|GetCurrentLevelName true))
      (bind _returnvalue_4 (Utilities|GetDataTableRow "/Game/BluePrint/DataTable_StageList.DataTable_StageList" (Utilities|String|StringToName _returnvalue_3))
        (:then
          (Pawn|Input|AddMovementInput (Math|Rotator|GetRotationXVector (Math|Rotator|FindLookatRotation (Transformation|GetActorLocation) (Math|Vector|MakeVector (.x (.GoalPos (Utilities|Struct|BreakStruct_StageLevelData _returnvalue_4))) (+ (.y _returnvalue) 2e+02) (.z _returnvalue)))) 1.0 false) ; 前に進む
          (CallFunction|移動方向に向く)
          (Utilities|FlowControl|DoOnce false ; 移動速度を下げる
            (:Completed
              (Variables|/Script/Engine.CharacterMovementComponent|SetMaxWalkSpeed (Variables|Character|GetCharacterMovement) 2e+02)))))
      (elif (not (Variables|Default|Getフラグ-衝突した))
        ;[1 1 1] 移動
        (Pawn|Input|AddMovementInput "0,1.000000, 0" 1.0 false) ; 前に進む
        (CallFunction|移動方向に向く)
        ;[1 1 1] ある程度落ちたらそこで停止
        (if (< (.z (Transformation|GetActorLocation)) (/ (Variables|Default|Getこれ以上落ちないZ座標) 2e+01))
          (Utilities|FlowControl|Sequence
            (:then_0
              (Utilities|FlowControl|DoOnce false
                (:Completed
                  (Audio|PlaySound2D "/Game/Sound/SE/ヒューンと落下_Cue.ヒューンと落下_Cue" 1.0 1.0 0.0 0 0))))
            (:then_1
              _)))
        (if (< (.z (Transformation|GetActorLocation)) (Variables|Default|Getこれ以上落ちないZ座標))
          (Rendering|SetVisibility (Variables|Character|GetMesh) false false)
          (Utilities|FlowControl|DoOnce false
            (:Completed
              (Pawn|Components|CharacterMovement|DisableMovement (Variables|Character|GetCharacterMovement)) ; ある程度落ちると停止
              (Variables|Default|Setフラグ-ミスした true))))
        (else
          ;[1 1 1] 衝突した後の挙動
          (Variables|Default|Set吹っ飛ばされてから何秒? (+ DeltaSeconds (Variables|Default|Get吹っ飛ばされてから何秒?))) ; 吹っ飛ばされてから何秒かをセットする
          (if (< (Variables|Default|Get吹っ飛ばされてから何秒?) 0.7) ; 吹っ飛ばされてから数秒立つと止まる
            (Transformation|SetActorRotation _ミスしたときの吹っ飛び方向)
            (Pawn|Input|AddMovementInput (Math|Vector|MakeVector (* (.x _returnvalue_2) -1.0) (* (.y _returnvalue_2) -1.0) (.z _returnvalue_2)) 1.0 true)
            ;;[1 1 1] 衝突した瞬間パラメータを変化させる
            (Utilities|FlowControl|DoOnce false
              (:Completed
                (Variables|/Script/Engine.CharacterMovementComponent|SetMaxWalkSpeed _charactermovement 3e+03)
                (Variables|/Script/Engine.CharacterMovementComponent|SetJumpZVelocity _charactermovement 5e+02)
                (Collision|SetCollisionEnabled (Variables|Collision|GetCapsuleComponent) "PhysicsOnly") ; コリジョンを無効化する
                (Character|Jump) ; 真後ろにジャンプする
                (Variables|/Script/Engine.CharacterMovementComponent|SetMaxAcceleration (Variables|Character|GetCharacterMovement) 4096.0)))
            (else
              ;;[1 1 1] ミスしてからしばらくたったら
              (Pawn|Components|CharacterMovement|DisableMovement (Variables|Character|GetCharacterMovement))
              (Variables|Default|Setフラグ-ミスした true))))))
    (else
      ;[1 1 1] スタート前は待機する
      (Transformation|SetActorRotation (Math|Rotator|FindLookatRotation (Math|Vector|MakeVector 0.0 0.0 0.0) (Math|Vector|MakeVector 0.0 1.0 0.0))) ; 前を向く
    )))

(event Input|AxisEvents|InputAxisMoveRight
  (params (AxisValue :type Float%20%28single-precision%29))
  ;[1 1 1] 横方向
  (if (Math|Boolean|ANDBoolean (not (Variables|Default|Getフラグ-衝突した)) (Variables|Default|Getフラグ-スタートしたか?) (not (Variables|Default|Getフラグ-ゴールした)))
    (Pawn|Input|AddMovementInput "-1.000000,0.000000, 0" AxisValue false)))

(event Input|AxisEvents|InputAxisMoveLeft
  (params (AxisValue :type Float%20%28single-precision%29))
  ;[1 1 1] 横方向
  (if (Math|Boolean|ANDBoolean (not (Variables|Default|Getフラグ-衝突した)) (Variables|Default|Getフラグ-スタートしたか?) (not (Variables|Default|Getフラグ-ゴールした)))
    (Pawn|Input|AddMovementInput "1.000000,0.000000, 0" AxisValue false)))

(fn ConstructionScript)

(fn Getフラグゴールした
  (return (Variables|Default|Getフラグ-ゴールした)))

(fn Getフラグ衝突した
  (return (Variables|Default|Getフラグ-衝突した)))

(fn 移動方向に向く
  (bind _returnvalue (Transformation|GetVelocity))
  (bind _returnvalue_2 (Math|Conversions|RotationFromXVector _returnvalue))
  (if (<= (Math|Vector|VectorLength _returnvalue) 3e+01) ; 停止しているならば前を向く
    (Transformation|SetActorRotation (Math|Rotator|FindLookatRotation (Math|Vector|MakeVector 0.0 0.0 0.0) (Math|Vector|MakeVector 0.0 1.0 0.0)))
    (else
      (Transformation|SetActorRotation _returnvalue_2) ; 移動方向からアクタの向きをセットする
    ))
  (Variables|Default|Setミスしたときの吹っ飛び方向 _returnvalue_2))

(fn 変速0~3
  (params (速度 :type Integer))
  (bind _charactermovement (Variables|Character|GetCharacterMovement))
  (switch int 速度
    (:Default
      (Variables|/Script/Engine.CharacterMovementComponent|SetMaxWalkSpeed _charactermovement 6.5e+02 :!label _label))
    (:0
      (Variables|/Script/Engine.CharacterMovementComponent|SetMaxWalkSpeed _charactermovement 5e+02))
    (:1
      (Variables|/Script/Engine.CharacterMovementComponent|SetMaxWalkSpeed _charactermovement 5.5e+02))
    (:2
      (Variables|/Script/Engine.CharacterMovementComponent|SetMaxWalkSpeed _charactermovement 6e+02))
    (:3
      (goto _label))
    (:4
      (Variables|/Script/Engine.CharacterMovementComponent|SetMaxWalkSpeed _charactermovement 1.5e+03))))