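; BP_Obstacle_Rolling_dachou is an obstacle actor that circles horizontally around its placed position at a configurable radius, angular speed and starting phase.
; BeginPlay sets the Obstacle tag, stores the spawn location as the orbit center and applies the initial angle.
; Each Tick advances the angle, moves the actor without sweeping via sine and cosine, and orients it along the radius, outward for non-negative speed and inward for negative speed.
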(event EventBeginPlay
  ;[1 1 1] 障害物タグをつける
  (Variables|Default|SetTags (Variables|コンポーネント|GetObstacle))
  ;[1 1 1] 回転の中心座標
  (Variables|Default|Setcenter_Pos (Transformation|GetActorLocation))
  (Variables|Default|Set現在の角度 (Variables|Default|Get初期位相)))

(event EventTick
  (params (DeltaSeconds :type Float%20%28single-precision%29))
  (bind _center_pos (Variables|Default|Getcenter_Pos))
  (bind _半径 (Variables|Default|Get半径))
  (bind _output_get (Variables|Default|Set現在の角度 (+ (* DeltaSeconds (Variables|Default|Get速度)) (Variables|Default|Get現在の角度))))
  (Transformation|SetActorLocation (Math|Vector|MakeVector (+ (* (Math|Trig|Cos(Degrees) _output_get) _半径) (.x _center_pos)) (+ (* (Math|Trig|Sin(Degrees) _output_get) _半径) (.y _center_pos)) (.z _center_pos)) false false)
  (if (>= (Variables|Default|Get速度) 0.0)
    (Transformation|SetActorRotation (Math|Rotator|FindLookatRotation (Variables|Default|Getcenter_Pos) (Transformation|GetActorLocation)) true)
    (else
      (Transformation|SetActorRotation (Math|Rotator|FindLookatRotation (Transformation|GetActorLocation) (Variables|Default|Getcenter_Pos)) true))))

(fn ConstructionScript)