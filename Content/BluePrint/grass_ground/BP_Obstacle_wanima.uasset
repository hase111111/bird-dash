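; BP_Obstacle_wanima is a moving obstacle actor that waits until the player character approaches along the Y axis.
; Tick compares the player's Y to its own minus a reaction-distance variable, then latches a movement flag.
; Once triggered, it slides toward negative Y by a fixed per-frame step, without sweep or delta-time scaling, and never stops.
; BeginPlay sets the actor's Tags; overlap handling is unused.
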(event EventBeginPlay
  (Variables|Default|SetTags (Variables|Default|GetTags_0)))

(event Collision|EventActorBeginOverlap
  (params (OtherActor :type Actor%20Object%20Reference)))

(event EventTick
  (params (DeltaSeconds :type Float%20%28single-precision%29))
  (bind _returnvalue (Transformation|GetActorLocation))
  (if (Variables|Default|Get移動開始)
    (Transformation|SetActorLocation (Math|Vector|MakeVector (.x _returnvalue) (+ (.y _returnvalue) -2.5) (.z _returnvalue)) false false)
    (elif (> (.y (Transformation|GetActorLocation (Game|GetPlayerCharacter 0))) (- (.y (Transformation|GetActorLocation)) (Variables|Default|Getどの程度で反応するかどうか)))
      (Variables|Default|Set移動開始 true))))

(fn ConstructionScript)