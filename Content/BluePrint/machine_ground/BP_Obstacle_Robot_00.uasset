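; Robot obstacle that homes in on the player, then charges in a straight line, triggered by the player's progress along the Y axis.
; Once the player passes 1300 units before the robot's Y, Tick turns it toward them horizontally and creeps it forward, storing that direction.
; Past 200 units before, it moves 15 units per frame along the stored direction, raising FloatingPawnMovement speed and playing a machine sound once.
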(event EventBeginPlay
  (Variables|/Script/Engine.FloatingPawnMovement|SetMaxSpeed (Variables|Default|GetFloatingPawnMovement) 5e+01)
  (Variables|Default|SetTags (Variables|Default|GetTags_0)))

(event Collision|EventActorBeginOverlap
  (params (OtherActor :type Actor%20Object%20Reference)))

(event EventTick
  (params (DeltaSeconds :type Float%20%28single-precision%29))
  (bind _returnvalue (Game|GetPlayerCharacter 0))
  (bind _returnvalue_2 (Transformation|GetActorLocation))
  (bind _returnvalue_3 (Transformation|GetActorLocation _returnvalue))
  (bind _returnvalue_4 (Math|Vector|MakeVector (.x _returnvalue_3) (.y _returnvalue_3) (.z _returnvalue_3)))
  (bind _returnvalue_5 (Math|Vector|MakeVector (.x _returnvalue_2) (.y _returnvalue_2) (.z _returnvalue_3)))
  (bind _returnvalue_6 (Math|Rotator|FindLookatRotation _returnvalue_5 _returnvalue_4))
  (bind _returnvalue_7 (Math|Rotator|GetRotationXVector _returnvalue_6))
  (if (< (- (.y (Transformation|GetActorLocation)) 1.3e+03) (.y (Transformation|GetActorLocation (Game|GetPlayerCharacter 0))))
    (if (< (- (.y (Transformation|GetActorLocation)) 2e+02) (.y (Transformation|GetActorLocation (Game|GetPlayerCharacter 0))))
      (Transformation|SetActorLocation (+ (* (Variables|Default|GetNewVar_0) 15.0) (Transformation|GetActorLocation)) false false)
      (Utilities|FlowControl|DoOnce false
        (:Completed
          (Variables|/Script/Engine.FloatingPawnMovement|SetMaxSpeed (Variables|Default|GetFloatingPawnMovement) 6.5e+02)
          (Audio|PlaySound2D "/Game/Sound/SE/機械音.機械音" 1.0 1.0 0.0 0 0)))
      (else
        (Transformation|SetActorLocation (+ (Transformation|GetActorLocation) _returnvalue_7) false false)
        (Transformation|SetActorRotation _returnvalue_6 true)
        (Variables|Default|SetNewVar_0 _returnvalue_7)))))

(fn ConstructionScript)