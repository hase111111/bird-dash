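; BP_Obstacle_Wrench is a wrench obstacle that starts at zero scale and activates based on the player's Y position.
; Tick compares Y distance against a threshold variable: within 1.2 times it, the wrench scales up with VInterpTo and plays its sound once.
; Within the threshold itself, it spins in yaw and travels along a direction variable in fixed per-frame steps, independent of delta time.
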(event EventBeginPlay
  (Transformation|SetActorScale3D "0, 0, 0")
  (Variables|Default|SetTags (Variables|Default|GetTags_0)))

(event EventTick
  (params (DeltaSeconds :type Float%20%28single-precision%29))
  (bind _returnvalue (Transformation|GetActorLocation))
  (bind _returnvalue_2 (Game|GetPlayerCharacter 0))
  (bind _returnvalue_3 (Transformation|GetActorLocation _returnvalue_2))
  (if (< (- (.y _returnvalue) (* (Variables|Default|Get反応位置) 1.2)) (.y _returnvalue_3))
    (Transformation|SetActorScale3D (Math|Interpolation|VInterpTo (Transformation|GetActorScale3D) "1.000000,1.000000,1.000000" (Utilities|Time|GetWorldDeltaSeconds) 5.0))
    (Utilities|FlowControl|Sequence
      (:then_0
        (Utilities|FlowControl|DoOnce false
          (:Completed
            (Audio|PlaySound2D "/Game/Sound/SE/スパナの音.スパナの音" 1.0 1.0 0.0 0 0))))
      (:then_1
        (if (< (- (.y _returnvalue) (Variables|Default|Get反応位置)) (.y _returnvalue_3)) :!label _label
          (Transformation|SetActorRotation (Math|Rotator|MakeRotator 0.0 0.0 (+ (Variables|Default|Get回転速度) (.yaw (Transformation|GetActorRotation)))))
          (Transformation|SetActorLocation (+ (* (Variables|Default|Get移動方向) 1e+01) (Transformation|GetActorLocation)) false false))))
    (else
      (goto _label))))

(fn ConstructionScript)