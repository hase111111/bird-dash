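; Yellow floor button that the player presses by overlapping its capsule, switching on the yellow state in the shared BP_Button_Controller.
; It finds the controller at BeginPlay, then polls its YellowON value every Tick.
; When that value changes, it swaps visibility between two static meshes to show the on or off look, so the button mirrors the controller's state.
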(event OnComponentBeginOverlap(Capsule)
  (params (OverlappedComponent :type Primitive%20Component%20Object%20Reference) (OtherActor :type Actor%20Object%20Reference) (OtherComp :type Primitive%20Component%20Object%20Reference) (OtherBodyIndex :type Integer) (bFromSweep :type Boolean) (SweepResult :type Hit%20Result%20Structure%20%28by%20ref%29))
  (bind _コントローラの参照 (Variables|Default|Getコントローラの参照))
  (Utilities|IsValid OtherActor
    (:Is%20Valid
      (if (Actor|ActorHasTag OtherActor "player")
        (Utilities|IsValid _コントローラの参照
          (:Is%20Valid
            (Default|SetYellowon _コントローラの参照)))))))

(event EventBeginPlay
  (bind _returnvalue (Actor|GetActorOfClass "/Game/BluePrint/machine_ground/BP_Button_Controller.BP_Button_Controller_C"))
  (bind _output_get (Variables|Default|Setコントローラの参照 _returnvalue))
  (bind _newparam (Default|GetYellowON _output_get))
  (bind _output_get_2 (Variables|Default|SetyellowON _newparam))
  (if _output_get_2
    (CallFunction|YellowONにする)
    (else
      (CallFunction|YellowOFFにする))))

(event EventTick
  (params (DeltaSeconds :type Float%20%28single-precision%29))
  (bind _コントローラの参照 (Variables|Default|Getコントローラの参照))
  (Utilities|IsValid _コントローラの参照
    (:Is%20Valid
      (bind _newparam (Default|GetYellowON _コントローラの参照))
      (if (Class|KismetMathLibrary|XORBoolean _newparam (Variables|Default|GetyellowON))
        (bind _output_get (Variables|Default|SetyellowON _newparam))
        (if _output_get
          (CallFunction|YellowONにする)
          (else
            (CallFunction|YellowOFFにする)))))))

(fn ConstructionScript)

(fn YellowONにする
  (Rendering|SetVisibility (Variables|Default|GetStaticMesh1) true false)
  (Rendering|SetVisibility (Variables|Default|GetStaticMesh) false false))

(fn YellowOFFにする
  (Rendering|SetVisibility (Variables|Default|GetStaticMesh1) false false)
  (Rendering|SetVisibility (Variables|Default|GetStaticMesh) true false))