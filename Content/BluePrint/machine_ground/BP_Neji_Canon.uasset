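; BP_Neji_Canon is a screw (neji) cannon projectile that plays a gunshot on spawn and flies to a set landing point.
; 着弾地点セット supplies the target XY, and Tick scales the screw toward full size while steering it horizontally via movement input, pitched 90 degrees.
; Near the target it rotates upright, then descends spinning in yaw to a fixed floor height, with a short lifespan set as descent begins.
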(event EventBeginPlay
  (Variables|Default|SetTags (Variables|Default|GetTags_0))
  (Audio|PlaySoundatLocation "/Game/Sound/SE/銃をうつ.銃をうつ" (Transformation|GetActorLocation) "0, 0, 0" 1.0 1.0 0.0 0 0 0 0))

(event EventTick
  (params (DeltaSeconds :type Float%20%28single-precision%29))
  (bind _returnvalue (Transformation|GetActorRotation))
  (bind _returnvalue_2 (Transformation|GetActorLocation))
  (bind _returnvalue_3 (Transformation|GetActorLocation))
  (bind _着弾地点x (Variables|Default|Get着弾地点X))
  (bind _着弾地点y (Variables|Default|Get着弾地点Y))
  (bind _returnvalue_4 (Math|Vector|MakeVector _着弾地点x _着弾地点y (.z _returnvalue_3)))
  (bind _returnvalue_5 (Math|Vector|MakeVector (.x _returnvalue_3) (.y _returnvalue_3) (.z _returnvalue_3)))
  (bind _returnvalue_6 (Math|Rotator|FindLookatRotation _returnvalue_5 _returnvalue_4))
  (bind (_roll _pitch _yaw) (Math|Rotator|BreakRotator _returnvalue_6))
  (Transformation|SetActorScale3D (* (Math|Vector|MakeVector 1.0 1.0 1.0) (Variables|Default|Get拡大率)))
  (if (<= (Variables|Default|Get拡大率) 1.0)
    (Variables|Default|Set拡大率 (Math|Interpolation|FInterptoConstant (Variables|Default|Get拡大率) 1.0 (Utilities|Time|GetWorldDeltaSeconds) 2.0)))
  (if (< (Math|Vector|VectorLength (- (Transformation|GetActorLocation) (Math|Vector|MakeVector (Variables|Default|Get着弾地点X) (Variables|Default|Get着弾地点Y) (.z (Transformation|GetActorLocation))))) 5e+01) ; 着弾地点に近づいたかどうか
    (if (and (< (.roll _returnvalue) 4.0) (< (.pitch _returnvalue) 4.0)) ; 下を向くまで待つ
      (if (< (.z (Transformation|GetActorLocation)) 5e+01) ; 墜ちる
        (Transformation|SetActorLocation (Math|Vector|MakeVector (.x _returnvalue_2) (.y _returnvalue_2) 5e+01) false false)
        (else
          (Pawn|Input|AddMovementInput (Math|Vector|MakeVector 0.0 0.0 -1.0) 1.0 false)))
      (Transformation|SetActorRotation (Math|Rotator|MakeRotator 0.0 0.0 (+ (.yaw (Transformation|GetActorRotation)) 1e+01)))
      (Utilities|FlowControl|DoOnce false
        (:Completed
          (Actor|SetLifeSpan 5.0)))
      (else
        (Transformation|SetActorRotation (Math|Interpolation|RInterpTo (Transformation|GetActorRotation) (Math|Rotator|MakeRotator 0.0 0.0 (.yaw (Transformation|GetActorRotation))) (Utilities|Time|GetWorldDeltaSeconds) 1e+01))))
    (else
      (Pawn|Input|AddMovementInput (Math|Rotator|GetRotationXVector _returnvalue_6) 1.0 false)
      (Transformation|SetActorRotation (Math|Rotator|MakeRotator _roll (+ _pitch 9e+01) _yaw)))))

(fn ConstructionScript)

(fn 着弾地点セット
  (params (ｘ :type Float%20%28double-precision%29) (ｙ :type Float%20%28double-precision%29))
  (Variables|Default|Set着弾地点X ｘ)
  (Variables|Default|Set着弾地点Y ｙ))