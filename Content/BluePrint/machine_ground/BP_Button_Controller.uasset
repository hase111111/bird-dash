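; BP_Button_Controller is a Blueprint that holds a shared on/off state, YellowON, for yellow button mechanics.
; On BeginPlay it sets YellowON from the 最初はyellowON initial-state flag.
; GetYellowON exposes the state, while SetYellowOn and SetYellowOff change it and play a 2D switch-change sound.
; It has no active overlap or tick logic, so changes come only through calls to its functions.
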(event EventBeginPlay
  (if (Variables|Default|Get最初はyellowON)
    (Variables|Default|Setyellow_ON true)
    (else
      (Variables|Default|Setyellow_ON false))))

(event Collision|EventActorBeginOverlap
  (params (OtherActor :type Actor%20Object%20Reference)))

(event EventTick
  (params (DeltaSeconds :type Float%20%28single-precision%29)))

(fn ConstructionScript)

(fn GetYellowON
  (return (Variables|Default|Getyellow_ON)))

(fn SetYellowon
  (Variables|Default|Setyellow_ON true)
  (Audio|PlaySound2D "/Game/Sound/SE/スイッチ変更.スイッチ変更" 1.0 1.0 0.0 0 0))

(fn SetYellowOff
  (Variables|Default|Setyellow_ON false)
  (Audio|PlaySound2D "/Game/Sound/SE/スイッチ変更.スイッチ変更" 1.0 1.0 0.0 0 0))