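; BP_Canon_Machine00 is a cannon machine that fires one BP_Neji_Canon AI pawn at the player.
; Each tick it yaws along the player-to-cannon direction, so its negative forward side faces the player.
; The first time the player's Y exceeds its own, a DoOnce spawns the pawn on that side.
; It then sets the pawn's landing point to the player's position, offset in Y by a look-ahead variable.
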(event Collision|EventActorBeginOverlap
  (params (OtherActor :type Actor%20Object%20Reference)))

(event EventTick
  (params (DeltaSeconds :type Float%20%28single-precision%29))
  (bind _returnvalue (Game|GetPlayerCharacter 0))
  (bind _returnvalue_2 (Game|GetPlayerCharacter 0))
  (bind _returnvalue_3 (Transformation|GetActorLocation))
  (bind _returnvalue_4 (Transformation|GetActorRotation))
  (bind _returnvalue_5 (Transformation|GetActorLocation _returnvalue_2))
  (Transformation|SetActorRotation (Math|Rotator|MakeRotator 0.0 0.0 (.yaw (Math|Rotator|FindLookatRotation (Transformation|GetActorLocation _returnvalue) (Transformation|GetActorLocation)))))
  (if (< (.y (Transformation|GetActorLocation)) (.y (Transformation|GetActorLocation _returnvalue)))
    (Utilities|FlowControl|DoOnce false
      (:Completed
        (bind _returnvalue_6 (AI|SpawnAIFromClass "/Game/BluePrint/machine_ground/BP_Neji_Canon.BP_Neji_Canon_C" 0 (+ (Math|Vector|MakeVector (* (Math|Trig|Cos(Degrees) (.yaw _returnvalue_4)) -75.0) (* (Math|Trig|Sin(Degrees) (.yaw _returnvalue_4)) -75.0) 0.0) (Math|Vector|MakeVector (.x _returnvalue_3) (.y _returnvalue_3) (+ (.z _returnvalue_3) 0.0))) "0, 0, 0" false 0))
        (bind _asbp_neji_canon (Utilities|Casting|CastToBP_Neji_Canon _returnvalue_6))
        (Default|着弾地点セット _asbp_neji_canon (.x _returnvalue_5) (+ (.y _returnvalue_5) (Variables|Default|Getプレイヤー前方Y)))))))

(fn ConstructionScript)