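; Stage game mode that sets up the camera, goal tape and heart pickups when a level begins.
; On BeginPlay it spawns BP_Player_Camera and makes it player 0's view target.
; It looks up the current level name in DataTable_StageList to place the goal tape, using a hardcoded position if no row exists.
; The same row positions three heart items, each given an index; none spawn without a row.
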(event EventBeginPlay
  ;[1 1 1] カメラを召喚しセットする
  (Game|SpawnActorfromClass "/Game/BluePrint/BP_Player_Camera.BP_Player_Camera_C" (Variables|Default|GetSpawn%20Transform) "Undefined" 0 0)
  (bind _returnvalue (Actor|GetActorOfClass "/Game/BluePrint/BP_Player_Camera.BP_Player_Camera_C"))
  (Game|Player|SetViewTargetwithBlend (Game|GetPlayerController 0) _returnvalue 0.0 "VTBlend_Linear" 0.0 false)
  ;[1 1 1] ゴールを生成する
  (bind _returnvalue_2 (Game|GetCurrentLevelName true))
  (bind _returnvalue_3 (Utilities|GetDataTableRow "/Game/BluePrint/DataTable_StageList.DataTable_StageList" (Utilities|String|StringToName _returnvalue_2))
    (:then
      (Game|SpawnActorfromClass "/Game/BluePrint/BP_GoalTape.BP_GoalTape_C" (Math|Transform|MakeTransform (.GoalPos (Utilities|Struct|BreakStruct_StageLevelData _returnvalue_3))) "Undefined" 0 0))
    (:RowNotFound
      (Game|SpawnActorfromClass "/Game/BluePrint/BP_GoalTape.BP_GoalTape_C" (Math|Transform|MakeTransform "0,10000.000000, 0") "Undefined" 0 0)))
  ;[1 1 1] ハートを追加
  (bind _returnvalue_4 (Game|GetCurrentLevelName true))
  (bind _returnvalue_5 (Utilities|GetDataTableRow "/Game/BluePrint/DataTable_StageList.DataTable_StageList" (Utilities|String|StringToName _returnvalue_4))
    (:then
      (bind _returnvalue_6 (Game|SpawnActorfromClass "/Game/BluePrint/BP_Item_Heart.BP_Item_Heart_C" (Math|Transform|MakeTransform (.Item1Pos (Utilities|Struct|BreakStruct_StageLevelData _returnvalue_5))) "Undefined" 0 0))
      (Default|番号を設定する _returnvalue_6)
      (bind _returnvalue_7 (Game|SpawnActorfromClass "/Game/BluePrint/BP_Item_Heart.BP_Item_Heart_C" (Math|Transform|MakeTransform (.Item2Pos (Utilities|Struct|BreakStruct_StageLevelData _returnvalue_5))) "Undefined" 0 0))
      (Default|番号を設定する _returnvalue_7 1)
      (bind _returnvalue_8 (Game|SpawnActorfromClass "/Game/BluePrint/BP_Item_Heart.BP_Item_Heart_C" (Math|Transform|MakeTransform (.Item3Pos (Utilities|Struct|BreakStruct_StageLevelData _returnvalue_5))) "Undefined" 0 0))
      (Default|番号を設定する _returnvalue_8 2))))

(event EventTick
  (params (DeltaSeconds :type Float%20%28single-precision%29)))

(fn ConstructionScript)