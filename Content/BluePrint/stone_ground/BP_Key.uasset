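; Collectible key actor, tagged Key, that follows the player once picked up.
; A randomly phased Tick counter wobbles its pitch while idle and drives a sine/cosine orbit around the player, smoothed with VInterpTo, after collection.
; A mesh overlap with a "player"-tagged actor triggers collection and a sound once.
; 上へあがり消えるフラグセット clears the tag and makes the collected key drift upward and sideways, expiring after a short lifespan.
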(event OnComponentBeginOverlap(StaticMesh)
  (params (OverlappedComponent :type Primitive%20Component%20Object%20Reference) (OtherActor :type Actor%20Object%20Reference) (OtherComp :type Primitive%20Component%20Object%20Reference) (OtherBodyIndex :type Integer) (bFromSweep :type Boolean) (SweepResult :type Hit%20Result%20Structure%20%28by%20ref%29))
  (Utilities|IsValid OtherActor
    (:Is%20Valid
      (if (Actor|ActorHasTag OtherActor "player")
        (Utilities|FlowControl|DoOnce false
          (:Completed
            (Variables|Default|Set所得済み true)
            (Audio|PlaySoundatLocation "/Game/Sound/SE/魔王魂_効果音_システム46_Cue.魔王魂_効果音_システム46_Cue" (Transformation|GetActorLocation) "0, 0, 0" 1.0 1.0 0.0 0 0 0 0)))))))

(event EventTick
  (params (DeltaSeconds :type Float%20%28single-precision%29))
  (bind _returnvalue (Game|GetPlayerCharacter 0))
  (bind _プレイヤーのr (Variables|Default|GetプレイヤーのR))
  (bind _returnvalue_2 (Transformation|GetActorLocation _returnvalue))
  (Variables|Default|Setcounter (+ DeltaSeconds (Variables|Default|Getcounter)))
  (if (Variables|Default|Get所得済み)
    (bind _output_get (Variables|Default|Set姿勢 (Math|Rotator|MakeRotator 0.0 0.0 (+ (Variables|Default|Get取得後の回転) (.yaw (Transformation|GetActorRotation))))))
    (Transformation|SetActorRotation _output_get)
    (if (not (Variables|Default|Get消える))
      (Transformation|SetActorLocation (Math|Interpolation|VInterpTo (Transformation|GetActorLocation) (Math|Vector|MakeVector (+ (* (Math|Trig|Sin(Radians) (* (Variables|Default|Getcounter) 5.0)) _プレイヤーのr) (.x _returnvalue_2)) (+ (* _プレイヤーのr (Math|Trig|Cos(Radians) (* (Variables|Default|Getcounter) 5.0))) (.y _returnvalue_2)) (.z _returnvalue_2)) (Utilities|Time|GetWorldDeltaSeconds) 2e+01) false false)
      (else
        (Transformation|SetActorLocation (+ (Transformation|GetActorLocation) (Math|Vector|MakeVector 0.0 2e+01 15.0)) false false)
        (Utilities|FlowControl|DoOnce false
          (:Completed
            (Actor|SetLifeSpan 5.0)))))
    (else
      (bind _output_get_2 (Variables|Default|Set姿勢 (Math|Rotator|MakeRotator 0.0 (+ 45.0 (* (Math|Trig|Sin(Radians) (* (Variables|Default|Getcounter) 5.0)) 1e+01)) 0.0)))
      (Transformation|SetActorRotation _output_get_2))))

(event EventBeginPlay
  (Variables|Default|Setcounter (* (Math|Random|RandomFloat) 3.6e+02))
  (Variables|Default|SetTags (Variables|Default|GetKey)))

(fn ConstructionScript)

(fn 上へあがり消えるフラグセット
  (Variables|Default|Set消える true)
  (Variables|Default|SetTags (Variables|Default|GetEmpty)))