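; BP_Gate_Key is an obstacle gate that sinks as keys are brought to it.
; Each "key"-tagged actor entering its Box raises the count and sink depth, and a BP_Key is told to rise and vanish.
; At three keys, a DoOnce clears the Obstacle tag, drops the gate further and plays a machine sound.
; Tick uses VInterpTo to ease the gate from its starting position down to the target depth.
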(event OnComponentBeginOverlap(Box)
  (params (OverlappedComponent :type Primitive%20Component%20Object%20Reference) (OtherActor :type Actor%20Object%20Reference) (OtherComp :type Primitive%20Component%20Object%20Reference) (OtherBodyIndex :type Integer) (bFromSweep :type Boolean) (SweepResult :type Hit%20Result%20Structure%20%28by%20ref%29))
  (Utilities|IsValid OtherActor
    (:Is%20Valid
      (if (Actor|ActorHasTag OtherActor "key")
        (bind _asbp_key (Utilities|Casting|CastToBP_Key OtherActor)
          (:then
            (Default|上へあがり消えるフラグセット _asbp_key))
          (:CastFailed
            _))
        (Variables|Default|Setカギの数 (+ (Variables|Default|Getカギの数) 1))
        (Variables|Default|Set目指す座標 (+ (Variables|Default|Get目指す座標) 5e+01))
        (if (>= (Variables|Default|Getカギの数) 3)
          (Utilities|FlowControl|DoOnce false
            (:Completed
              (Variables|Default|SetTags (Variables|Default|Getempty))
              (Variables|Default|Set目指す座標 (+ (Variables|Default|Get目指す座標) 1.1e+02))
              (Audio|PlaySound2D "/Game/Sound/SE/機械音.機械音" 1.0 1.0 0.0 0 0))))))))

(event EventBeginPlay
  (Variables|Default|SetTags (Variables|Default|Getobstacle))
  (Variables|Default|Set初期座標 (Transformation|GetActorLocation)))

(event EventTick
  (params (DeltaSeconds :type Float%20%28single-precision%29))
  (bind _初期座標 (Variables|Default|Get初期座標))
  (Transformation|SetActorLocation (Math|Interpolation|VInterpTo (Transformation|GetActorLocation) (Math|Vector|MakeVector (.x _初期座標) (.y _初期座標) (- (.z _初期座標) (Variables|Default|Get目指す座標))) (Utilities|Time|GetWorldDeltaSeconds) 1e+01) false false))

(fn ConstructionScript)