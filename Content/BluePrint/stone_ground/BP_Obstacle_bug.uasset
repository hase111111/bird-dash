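; BP_Obstacle_bug is a crawling bug obstacle pawn that stays still until the player approaches.
; At BeginPlay it stores its facing as the move direction and applies its speed to the FloatingPawnMovement component.
; Each tick, once the player's Y passes an activation offset before its own, it moves straight along that direction.
; The first movement starts a five-second lifespan and plays a cockroach scuttling sound once.
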(event EventBeginPlay
  (Variables|Default|SetTags (Variables|Default|GetTags_0))
  (Variables|Default|Set移動する方向 (Math|Rotator|GetRotationXVector (Transformation|GetActorRotation)))
  (Variables|/Script/Engine.FloatingPawnMovement|SetMaxSpeed (Variables|Default|GetFloatingPawnMovement) (Variables|Default|Get移動速度)))

(event EventTick
  (params (DeltaSeconds :type Float%20%28single-precision%29))
  (bind _returnvalue (Game|GetPlayerCharacter 0))
  (bind _移動する方向 (Variables|Default|Get移動する方向))
  ;[1 1 1] キャラクターが近づくまで動かない
  (Utilities|IsValid _returnvalue
    (:Is%20Valid
      (if (> (.y (Transformation|GetActorLocation _returnvalue)) (- (.y (Transformation|GetActorLocation)) (Variables|Default|Getいつ起動するかy)))
        ;[1 1 1] 移動する
        (Transformation|SetActorRotation (Math|Conversions|RotationFromXVector _移動する方向))
        (Pawn|Input|AddMovementInput _移動する方向 1.0 false)
        ;[1 1 1] 動き始めてから一定時間で消滅
        (Utilities|FlowControl|DoOnce false
          (:Completed
            (Actor|SetLifeSpan 5.0)
            (Audio|PlaySound2D "/Game/Sound/SE/ゴキがカサカサ・・・_Cue.ゴキがカサカサ・・・_Cue" 1.0 1.0 0.0 0 0)))))))

(fn ConstructionScript)