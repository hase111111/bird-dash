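; BP_Confuser is an actor that keeps turning to face the player while wobbling.
; On BeginPlay it sets its Tags from the Tags0 variable.
; Each Tick it takes the look-at yaw toward player pawn 0 with a fixed offset, keeps its roll, and drives pitch with mixed sine and cosine waves of accumulated time for an irregular sway.
; The overlap event is an unused stub.
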(event EventBeginPlay
  (Variables|Default|SetTags (Variables|Default|GetTags_0)))

(event Collision|EventActorBeginOverlap
  (params (OtherActor :type Actor%20Object%20Reference)))

(event EventTick
  (params (DeltaSeconds :type Float%20%28single-precision%29))
  (bind _output_get (Variables|Default|Set経過時間 (+ DeltaSeconds (Variables|Default|Get経過時間))))
  (Transformation|SetActorRotation (Math|Rotator|MakeRotator (.roll (Transformation|GetActorRotation)) (* (+ (Math|Trig|Sin(Radians) (* _output_get 3.0)) (Math|Trig|Cos(Radians) (* _output_get 5.0))) 3e+01) (+ (.yaw (Math|Rotator|FindLookatRotation (Transformation|GetActorLocation) (Transformation|GetActorLocation (Game|Player|GetPlayerPawn 0)))) 2.7e+02))))

(fn ConstructionScript)