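; BP_GoalTape is a goal tape actor that rises when the player touches it.
; On BeginPlay it tags itself Goal, faces negative X, snaps to a fixed height and disables its tick.
; An overlap on its StaticMesh by a Player-tagged actor enables tick, which raises the tape at the 上昇z速度 (rise speed) rate until it is about 200 units above its start height.
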(event OnComponentBeginOverlap(StaticMesh)
  (params (OverlappedComponent :type Primitive%20Component%20Object%20Reference) (OtherActor :type Actor%20Object%20Reference) (OtherComp :type Primitive%20Component%20Object%20Reference) (OtherBodyIndex :type Integer) (bFromSweep :type Boolean) (SweepResult :type Hit%20Result%20Structure%20%28by%20ref%29))
  (Utilities|IsValid OtherActor
    (:Is%20Valid
      (if (Actor|ActorHasTag OtherActor (Variables|Default|GetPlayer))
        (Actor|Tick|SetActorTickEnabled true)))))

(event EventBeginPlay
  (bind _returnvalue (Transformation|GetActorLocation))
  (Variables|Default|SetTags (Variables|Default|GetGoal))
  (Transformation|SetActorRotation (Math|Rotator|MakeRotfromX (Math|Vector|MakeVector -1.0 0.0 0.0)))
  (Transformation|SetActorLocation (Math|Vector|MakeVector (.x _returnvalue) (.y _returnvalue) 5e+01) false false)
  (Variables|Default|SetfirstZ (.z (Transformation|GetActorLocation)))
  (Actor|Tick|SetActorTickEnabled false))

(event EventTick
  (params (DeltaSeconds :type Float%20%28single-precision%29))
  (bind _returnvalue (Transformation|GetActorLocation))
  (if (> (+ (Variables|Default|GetfirstZ) 2e+02) (.z (Transformation|GetActorLocation)))
    (Transformation|SetActorLocation (Math|Vector|MakeVector (.x _returnvalue) (.y _returnvalue) (+ (* DeltaSeconds (Variables|Default|Get上昇z速度)) (.z _returnvalue))) false false)))

(fn ConstructionScript)